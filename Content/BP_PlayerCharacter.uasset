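; BP_PlayerCharacter is the player character Blueprint, handling health bar setup and a key-triggered damage call.
; BeginPlay creates the WBP_PlayerHealthbar widget for the first player controller and adds it to the viewport.
; Pressing Q fetches the player character and calls its TakeDamage event, which passes a fixed damage amount to DamageHealth on WizardGameState.
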(event `self.ReceiveBeginPlay`
  (bind _returnvalue (`|CreateWidget` "/Game/UI/Player/WBP_PlayerHealthbar.WBP_PlayerHealthbar_C" (`GameplayStatics.GetPlayerController` 0)))
  (`UserWidget.AddToViewport` _returnvalue 0))

(event `Key|Q`
  (params (Key :type "Key Structure"))
  (:`Pressed`
    (bind _asbp_player_character (cast `/Game/BP_PlayerCharacter` (`GameplayStatics.GetPlayerCharacter` 0)))
    (`self.TakeDamage` _asbp_player_character)))

(event `TakeDamage`
  (bind _aswizard_game_state (cast `WizardGameState` (`GameplayStatics.GetGameState`)))
  (`WizardGameState.DamageHealth` _aswizard_game_state 10.0))

(fn `UserConstructionScript`)