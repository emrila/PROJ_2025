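; BP_MageCharacter is the player mage, which creates the health bar widget and shows the profile username on a text render at BeginPlay.
; Overlapping a BP_Mushroom launches it away from the mushroom, calls TakeDamage on BP_MageController and sets an i-frame flag that a one-second timer clears.
; The i-frame check is disconnected, so the flag does not block repeat hits.
; Q jumps into the same hit logic, bypassing the mushroom cast.
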(event `self.ReceiveBeginPlay`
  (bind (_returnvalue_steamid _returnvalue_username) (break `PlayerProfile` (`PlayerLoginSystem.GetProfile` (subsystem `PlayerLoginSystem`))))
  (bind _returnvalue (`|CreateWidget` "/Game/UI/Player/WBP_PlayerHealthbar.WBP_PlayerHealthbar_C" (`GameplayStatics.GetPlayerController` 0)))
  (`UserWidget.AddToViewport` _returnvalue 0)
  (`TextRenderComponent.K2_SetText` (`self.TextRender`) (`KismetTextLibrary.Conv_StringToText` _returnvalue_username)))

(event `self.ReceiveActorBeginOverlap`
  (params (OtherActor :type "Actor Object Reference"))
  (bind _asbp_mushroom (cast `/Game/Enemy/BP_Mushroom` OtherActor))
  (cast `MageCharacter` (`GameplayStatics.GetPlayerCharacter` 0) :!label _label)
  (bind (_returnvalue_x _returnvalue_y) (`KismetMathLibrary.BreakVector` (* (`KismetMathLibrary.Normal` (- (`self.K2_GetActorLocation` _asbp_mushroom) (`self.K2_GetActorLocation`))) -1000.0)))
  (`self.LaunchCharacter` (`KismetMathLibrary.MakeVector` _returnvalue_x _returnvalue_y 100.0))
  (bind _asbp_mage_controller (cast `/Game/Basir/BP_MageController` (`self.GetLocalViewingPlayerController` self)))
  (`/Game/Basir/BP_MageController.TakeDamage` _asbp_mage_controller)
  (set `self.HasIframes` true)
  (`KismetSystemLibrary.K2_SetTimer` null "ResetIframes" 1.0))

(event `ResetIframes`
  (set `self.HasIframes` false))

(event `Key|Q`
  (params (Key :type "Key Structure"))
  (:`Pressed`
    (goto _label)))

(event `self.ReceiveTick`
  (params (DeltaSeconds :type "Float (single-precision)")))

(fn `UserConstructionScript`)