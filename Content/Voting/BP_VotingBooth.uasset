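; BP_VotingBooth is a voting booth actor that shows a set of candidates in a widget.
; On BeginPlay it converts each entry in Choices into a Candidates record with a zeroed first field plus class, description, row name and modifier data.
; It then creates a WBP_Voting widget with a reference to itself, has it show the candidates and assigns it to its Widget component.
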(event `self.ReceiveBeginPlay`
  (for _array_element (`self.Choices`)
    (`self.CreateCandidate` _array_element))
  (`self.SpawnWidget`))

(event `CreateCandidate`
  (params (Candidate :type "Candidate Structure"))
  (`KismetArrayLibrary.Array_Add` (`self.Candidates`) (make `Candidate` 0 Candidate_CandidateClass Candidate_Description Candidate_RowName Candidate_ModifierData)))

(event `SpawnWidget`
  (bind _returnvalue (`|CreateWidget` "/Game/UI/WorldSpace/WBP_Voting.WBP_Voting_C" null self))
  (bind _output_get (set `self.VotingWidget` _returnvalue))
  (`/Game/UI/WorldSpace/WBP_Voting.ShowCandidates` _output_get)
  (set `/Game/UI/WorldSpace/WBP_Voting.Booth` self _output_get)
  (`WidgetComponent.SetWidget` (`self.Widget`) _output_get))

(fn `UserConstructionScript`)