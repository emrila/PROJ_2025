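; A widget component that shows an enemy's health bar in world space and keeps it facing the player's camera.
; On BeginPlay it requires an EnemyBase owner, uses a custom draw size for Golems, and passes the owner to its WBP_EnemyHealthbar widget.
; A fast looping timer, rather than Tick, then rotates the component toward the first player's camera for a billboard effect.
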(event `self.ReceiveBeginPlay`
  (bind _asenemy_base (cast `EnemyBase` (`self.GetOwner`)))
  (cast `/Game/Enemy/Golem/BP_Golem` _asenemy_base
    (:`then`
      (`self.SetDrawSize` (250.0 5.0)))
    (:`CastFailed`
      _))
  (bind _aswbp_enemy_healthbar (cast `/Game/Enemy/WBP_EnemyHealthbar` (`self.GetWidget`)))
  (set `/Game/Enemy/WBP_EnemyHealthbar.Owner` _asenemy_base _aswbp_enemy_healthbar)
  (`KismetSystemLibrary.K2_SetTimer` null "AdjustWidget" 0.01 true true))

(event `AdjustWidget`
  (`self.K2_SetWorldRotation` (`KismetMathLibrary.FindLookAtRotation` (`self.K2_GetComponentLocation`) (`self.K2_GetComponentLocation` (`PlayerCameraManager.TransformComponent` (`GameplayStatics.GetPlayerCameraManager` 0))))))