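; BP_CookingPot is an interactable cooking pot that lets the player open the inventory to select items.
; Its sphere overlap shows a "press E to cook" prompt for the locally controlled player character and removes it on exit.
; PlayerPressedE, with no caller in this file, swaps a visible prompt for WBP_Inventory in item selection mode and ignores player 0's move and look input, without restoring it here.
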(event `self.Sphere.OnComponentBeginOverlap`
  (params (OverlappedComponent :type "PrimitiveComponent Object Reference") (OtherActor :type "Actor Object Reference") (OtherComp :type "PrimitiveComponent Object Reference") (OtherBodyIndex :type Integer) (bFromSweep :type Boolean) (SweepResult :type "HitResult Structure (by ref)"))
  (bind _asplayer_character_base (cast `PlayerCharacterBase` OtherActor))
  (if (`Pawn.IsLocallyControlled` _asplayer_character_base)
    (if (not (`KismetSystemLibrary.IsValid` (`self.EToCookWidget`)))
      (bind _returnvalue (`|CreateWidget` "/Game/UI/WBP_EToCook.WBP_EToCook_C"))
      (bind _output_get (set `self.EToCookWidget` _returnvalue))
      (`UserWidget.AddToViewport` _output_get 0))))

(event `self.Sphere.OnComponentEndOverlap`
  (params (OverlappedComponent :type "PrimitiveComponent Object Reference") (OtherActor :type "Actor Object Reference") (OtherComp :type "PrimitiveComponent Object Reference") (OtherBodyIndex :type Integer))
  (bind _etocookwidget (`self.EToCookWidget`))
  (bind _asplayer_character_base (cast `PlayerCharacterBase` OtherActor))
  (if (`Pawn.IsLocallyControlled` _asplayer_character_base)
    (if (`KismetSystemLibrary.IsValid` _etocookwidget)
      (if (`Widget.IsInViewport` _etocookwidget)
        (`Widget.RemoveFromParent` (`self.EToCookWidget`))
        (set `self.EToCookWidget` null)))))

(event `PlayerPressedE`
  (bind _returnvalue (`GameplayStatics.GetPlayerController` 0))
  (bind _etocookwidget (`self.EToCookWidget`))
  (if (`KismetSystemLibrary.IsValid` _etocookwidget)
    (if (`Widget.IsInViewport` _etocookwidget)
      (`Widget.RemoveFromParent` (`self.EToCookWidget`))
      (set `self.EToCookWidget` null)
      (`Controller.SetIgnoreMoveInput` _returnvalue true)
      (`Controller.SetIgnoreLookInput` _returnvalue true)
      (bind _returnvalue_2 (`|CreateWidget` "/Game/UI/WBP_Inventory.WBP_Inventory_C"))
      (set `InventoryWidget.ItemSelectionMode` true _returnvalue_2)
      (`UserWidget.AddToViewport` _returnvalue_2 0))))

(fn `UserConstructionScript`)