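; BP_CactusProjectile is the cactus enemy's projectile actor, which damages the player character on overlap.
; Its Box component takes the Projectile collision profile in both the construction script and BeginPlay, and the actor destroys itself after a short delay.
; Overlaps apply scaled base damage with the owner as causer and the player's local viewing controller as instigator, without destroying the projectile.
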(event `self.ReceiveBeginPlay`
  (`PrimitiveComponent.SetCollisionProfileName` (`self.Box`) "Projectile" true)
  (`KismetSystemLibrary.Delay` 5.0)
  (`self.K2_DestroyActor`))

(event `self.ReceiveActorBeginOverlap`
  (params (OtherActor :type "Actor Object Reference"))
  (bind _asbp_player_character_base (cast `/Game/Developer/Basir/BP_PlayerCharacterBase` OtherActor))
  (`GameplayStatics.ApplyDamage` _asbp_player_character_base (* (`self.Base Damage`) (`self.DamageMultiplier`)) (`Pawn.GetLocalViewingPlayerController` _asbp_player_character_base) (`self.GetOwner`) "/Script/Engine.DamageType"))

(fn `UserConstructionScript`
  (`PrimitiveComponent.SetCollisionProfileName` (`self.Box`) "Projectile" true))