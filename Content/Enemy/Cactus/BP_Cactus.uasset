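; Cactus enemy Blueprint that provides the visual feedback for a spike indicator and for taking hits.
; SpikeIndicator plays a timeline that scales the static mesh, with one track for X and Y and another for Z.
; The construction script stores dynamic instances of every mesh material, which HitFeedback briefly flashes through the DamageToggle parameter.
; SetMat swaps the slot 0 material without updating that stored array.
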(event `self.ReceiveBeginPlay`)

(event `SpikeIndicator`
  (bind (_direction _newtrack_0 _newtrack_1) (`Timeline|Timeline` :!via `PlayFromStart`)
    (:`Update`
      (`SceneComponent.SetRelativeScale3D` (`self.StaticMesh`) (`KismetMathLibrary.MakeVector` _newtrack_1 _newtrack_1 _newtrack_0)))))

(event `self.HitFeedback`
  (for _array_element (`self.DynamicMaterials`)
    (`MaterialInstanceDynamic.SetScalarParameterValue` _array_element "DamageToggle" 1.0))
  (`KismetSystemLibrary.Delay` 0.1)
  (for _array_element_2 (`self.DynamicMaterials`)
    (`MaterialInstanceDynamic.SetScalarParameterValue` _array_element_2 "DamageToggle" 0.0)))

(fn `MakeDynamicMaterial`
  (bind _staticmesh (`self.StaticMesh`))
  (for (_array_element _array_index) (`MeshComponent.GetMaterials` (`self.StaticMesh`))
    (bind _returnvalue (`PrimitiveComponent.CreateDynamicMaterialInstance` _staticmesh _array_index _array_element "None"))
    (`PrimitiveComponent.SetMaterial` _staticmesh _array_index _returnvalue)
    (`KismetArrayLibrary.Array_Add` (`self.DynamicMaterials`) _returnvalue)))

(fn `SetMat`
  (params (MatToReplace :type "Material Object Reference"))
  (bind _staticmesh (`self.StaticMesh`))
  (`PrimitiveComponent.SetMaterial` _staticmesh 0 MatToReplace)
  (`PrimitiveComponent.SetMaterial` _staticmesh 0 MatToReplace))

(fn `UserConstructionScript`
  (`self.MakeDynamicMaterial`))