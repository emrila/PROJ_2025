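; Falling carrot hazard that drops near a random player, damaging what it hits.
; The server places it overhead or at blocking geometry, then self-rearming timers lower it while shaking, drop it spinning, and sink it underground before destruction.
; Landing, detected by a short line trace, spawns a BP_Shockwave.
; Box overlap damages each player once with a multicast mesh spin, and deals heavy ChronoRiftDamageType damage to enemies.
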(event `Shake`
  (bind (_returnvalue_x _returnvalue_y _returnvalue_z) (`KismetMathLibrary.BreakVector` (`self.K2_GetActorLocation`)))
  (bind (_returnvalue_x_2 _returnvalue_y_2 _returnvalue_z_2) (`KismetMathLibrary.BreakVector` (`self.K2_GetActorLocation`)))
  (bind (_start_x _start_y) (`KismetMathLibrary.BreakVector` (`self.Start`)))
  (bind (_start_x_2 _start_y_2) (`KismetMathLibrary.BreakVector` (`self.Start`)))
  (`self.K2_SetActorLocation` (`KismetMathLibrary.MakeVector` (+ _start_x_2 (`KismetMathLibrary.RandomFloatInRange` -3.0 3.0)) (+ _start_y_2 (`KismetMathLibrary.RandomFloatInRange` -3.0 3.0)) _returnvalue_z))
  (if (`self.StopShake`)
    (`self.K2_SetActorLocation` (`KismetMathLibrary.MakeVector` _start_x _start_y _returnvalue_z_2))
    (else
      (`KismetSystemLibrary.K2_SetTimer` null "Shake" 0.01))))

(event `Rotate`
  (bind (_returnvalue_roll _returnvalue_pitch _returnvalue_yaw) (`KismetMathLibrary.BreakRotator` (`self.K2_GetActorRotation`)))
  (`self.K2_SetActorRotation` (`KismetMathLibrary.MakeRotator` 0.0 0.0 (+ _returnvalue_yaw (`self.RotateSpeed`))))
  (`KismetSystemLibrary.K2_SetTimer` null "Rotate" 0.01))

(event `self.ReceiveBeginPlay`
  (bind _end (`self.End`))
  (`/Engine/EditorBlueprintResources/ActorMacros.Switch Has Authority`
    (:`Authority`
      (set `self.End` (+ (`NavigationSystemV1.K2_GetRandomReachablePointInRadius` (`self.K2_GetActorLocation` (`PlayerState.GetPawn` (`KismetArrayLibrary.Array_Random` (`GameStateBase.PlayerArray` (`GameplayStatics.GetGameState`))))) 2500.0 null null) (0.0 0.0 3500.0)))
      (bind _outhit (`KismetSystemLibrary.LineTraceSingleForObjects` (- _end (0.0 0.0 3400.0)) _end (`|MakeArray` "ObjectTypeQuery1" :!type "EObjectTypeQuery Enum")))
      (bind (_bblockinghit _binitialoverlap _time _distance _location _impactpoint) (`GameplayStatics.BreakHitResult` _outhit))
      (if _bblockinghit
        (`self.K2_SetActorLocation` _impactpoint)
        (else
          (`self.K2_SetActorLocation` (`self.End`))))
      (set `self.LerpAlpha` 0.0)
      (set `self.Start` (`self.K2_GetActorLocation`))
      (`KismetSystemLibrary.K2_SetTimer` null "LerpDownwards" 0.01)
      (`KismetSystemLibrary.K2_SetTimer` null "Shake" 0.05))))

(event `LerpDownwards`
  (bind (_returnvalue_x _returnvalue_y) (`KismetMathLibrary.BreakVector` (`self.K2_GetActorLocation`)))
  (bind (_returnvalue_x_2 _returnvalue_y_2 _returnvalue_z) (`KismetMathLibrary.BreakVector` (`KismetMathLibrary.VLerp` (`self.Start`) (- (`self.Start`) (0.0 0.0 470.0)) (`self.LerpAlpha`))))
  (`self.K2_SetActorLocation` (`KismetMathLibrary.MakeVector` _returnvalue_x _returnvalue_y _returnvalue_z))
  (bind _output_get (set `self.LerpAlpha` (+ (`self.LerpAlpha`) 0.0025)))
  (if (>= _output_get 1.0)
    (`KismetSystemLibrary.Delay` 1.0)
    (set `self.StopShake` true)
    (`KismetSystemLibrary.K2_SetTimer` null "Fall" 0.01)
    (`KismetSystemLibrary.K2_SetTimer` null "Rotate" 0.01)
    (else
      (`KismetSystemLibrary.K2_SetTimer` null "LerpDownwards" 0.01))))

(event `self.Box.OnComponentBeginOverlap`
  (params (OverlappedComponent :type "PrimitiveComponent Object Reference") (OtherActor :type "Actor Object Reference") (OtherComp :type "PrimitiveComponent Object Reference") (OtherBodyIndex :type Integer) (bFromSweep :type Boolean) (SweepResult :type "HitResult Structure (by ref)"))
  (`/Engine/EditorBlueprintResources/ActorMacros.Switch Has Authority`
    (:`Authority`
      (bind _asbp_player_character_base (cast `/Game/Developer/Basir/BP_PlayerCharacterBase` OtherActor)
        (:`then`
          (if (not (`KismetArrayLibrary.Array_Contains` (`self.HitPlayers`) _asbp_player_character_base))
            (`KismetArrayLibrary.Array_Add` (`self.HitPlayers`) _asbp_player_character_base)
            (`GameplayStatics.ApplyDamage` _asbp_player_character_base 150.0)
            (`self.MulticastSpin` _asbp_player_character_base)))
        (:`CastFailed`
          (bind _asenemy_base (cast `EnemyBase` OtherActor))
          (`GameplayStatics.ApplyDamage` _asenemy_base 1000.0 null null "/Script/PROJ_2025.ChronoRiftDamageType"))))))

(event `Fall`
  (bind (_returnvalue_x _returnvalue_y _returnvalue_z) (`KismetMathLibrary.BreakVector` (`self.K2_GetActorLocation`)))
  (bind _returnvalue (`self.K2_GetActorLocation`))
  (`self.K2_SetActorLocation` (`KismetMathLibrary.MakeVector` _returnvalue_x _returnvalue_y (- _returnvalue_z 16.0)))
  (bind (_outhit _returnvalue_2) (`KismetSystemLibrary.LineTraceSingleForObjects` (+ _returnvalue (0.0 0.0 90.0)) (+ _returnvalue (0.0 0.0 70.0)) (`|MakeArray` "ObjectTypeQuery1" :!type "EObjectTypeQuery Enum")))
  (if _returnvalue_2
    (set `self.Start` (`self.K2_GetActorLocation`))
    (set `self.RotateSpeed` 20.0)
    (set `self.LerpAlpha` 0.0)
    (bind _returnvalue_3 (`|SpawnActorFromClass` "/Game/Enemy/MossGolem/BP_Shockwave.BP_Shockwave_C" (`KismetMathLibrary.MakeTransform` (+ (`self.K2_GetActorLocation`) (0.0 0.0 130.0))) "Undefined" "MultiplyWithRoot" null null))
    (set `EnemySubAttack.DamageMultiplier` 1.5 _returnvalue_3)
    (`KismetSystemLibrary.Delay` 0.5)
    (`KismetSystemLibrary.K2_SetTimer` null "Dig" 0.01)
    (else
      (`KismetSystemLibrary.K2_SetTimer` null "Fall" 0.01))))

(event `MulticastSpin`
  (params (PlayerToSpin :type "/Game/Developer/Basir/BP_PlayerCharacterBase Object Reference"))
  (bind (_direction _newtrack_0) (`Timeline|Spin` :!via `PlayFromStart`)
    (:`Update`
      (`SceneComponent.K2_SetRelativeRotation` (`Character.Mesh` PlayerToSpin) (`KismetMathLibrary.MakeRotator` 0.0 0.0 (- _newtrack_0 90.0)) false false))))

(event `Dig`
  (bind (_returnvalue_x _returnvalue_y) (`KismetMathLibrary.BreakVector` (`self.K2_GetActorLocation`)))
  (bind (_returnvalue_x_2 _returnvalue_y_2 _returnvalue_z) (`KismetMathLibrary.BreakVector` (`KismetMathLibrary.VLerp` (`self.Start`) (- (`self.Start`) (0.0 0.0 2200.0)) (`self.LerpAlpha`))))
  (`self.K2_SetActorLocation` (`KismetMathLibrary.MakeVector` _returnvalue_x _returnvalue_y _returnvalue_z))
  (bind _output_get (set `self.LerpAlpha` (+ (`self.LerpAlpha`) 0.0065)))
  (if (>= _output_get 1.0)
    (`KismetSystemLibrary.Delay` 8.0)
    (`self.K2_DestroyActor`)
    (else
      (`KismetSystemLibrary.K2_SetTimer` null "Dig" 0.01))))

(fn `UserConstructionScript`)