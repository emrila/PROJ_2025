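; BP_Mushroom is a mushroom enemy whose FootSteps component shows only while its AI is allowed to attack.
; One second after BeginPlay, it casts its controller to BP_MushroomAIController and caches that controller's Blackboard.
; Each Tick, once the Blackboard is valid, it polls the CanAttack bool and sets FootSteps visibility to match.
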(event `self.ReceiveBeginPlay`
  (`KismetSystemLibrary.Delay` 1.0)
  (bind _asbp_mushroom_aicontroller (cast `/Game/Enemy/BP_MushroomAIController` (`AIBlueprintHelperLibrary.GetAIController` self)))
  (set `self.Blackboard` (`AIBlueprintHelperLibrary.GetBlackboard` _asbp_mushroom_aicontroller)))

(event `self.ReceiveTick`
  (params (DeltaSeconds :type "Float (single-precision)"))
  (bind _blackboard (`self.Blackboard`))
  (bind _footsteps (`self.FootSteps`))
  (if (`KismetSystemLibrary.IsValid` _blackboard)
    (if (`BlackboardComponent.GetValueAsBool` _blackboard "CanAttack")
      (`SceneComponent.SetVisibility` _footsteps true false)
      (else
        (`SceneComponent.SetVisibility` _footsteps false false)))))

(fn `UserConstructionScript`)