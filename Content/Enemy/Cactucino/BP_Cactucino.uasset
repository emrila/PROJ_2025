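; Cactucino boss enemy that rises from underground, spawns goons at four points, then starts its behavior tree.
; Provides dig, burst, rotating fan-fire and spike explosion events, using timelines for mesh height and yaw.
; HitFeedback flashes dynamic materials and flags the FanAttack blackboard key at health thresholds.
; Head and body hitboxes damage and launch players unless digging; death triggers loot through the boss room manager.
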(event `self.HitFeedback`
  (bind _thresholds (`self.Thresholds`))
  (bind _output (`|GetArrayItem` _thresholds (`KismetArrayLibrary.Array_LastIndex` _thresholds)))
  (for _array_element (`self.Dynamic Materials`)
    (`MaterialInstanceDynamic.SetScalarParameterValue` _array_element "DamageToggle" 1.0))
  (`KismetSystemLibrary.Delay` 0.1)
  (for _array_element_2 (`self.Dynamic Materials`)
    (`MaterialInstanceDynamic.SetScalarParameterValue` _array_element_2 "DamageToggle" 0.0)
    (if (< (`self.Health`) (* (`self.MaxHealth`) _output))
      (`KismetSystemLibrary.PrintString` "Threshold reached")
      (`BlackboardComponent.SetValueAsBool` (`AIController.Blackboard` (`AIBlueprintHelperLibrary.GetAIController` self)) "FanAttack" true)
      (`KismetArrayLibrary.Array_RemoveItem` (`self.Thresholds`) _output))))

(event `DigUp`
  (`SceneComponent.K2_SetRelativeLocation` (`self.Mesh`) (0.0 0.0 -300.0) false false)
  (`KismetSystemLibrary.Delay` 5.0)
  (bind (_direction _height) (`Timeline|Timeline` :!via `PlayFromStart`)
    (:`Update`
      (`SceneComponent.K2_SetRelativeLocation` (`self.Mesh`) (`KismetMathLibrary.MakeVector` 0.0 0.0 _height) false false))
    (:`Finished`
      (`KismetSystemLibrary.Delay` 0.4)
      (`self.SpawnGoons`)
      (`KismetSystemLibrary.Delay` 4.0)
      (`AIController.RunBehaviorTree` (`AIBlueprintHelperLibrary.GetAIController` self) "/Game/Enemy/Cactucino/BT_Cactucino.BT_Cactucino")
      (`BlackboardComponent.SetValueAsVector` (`AIBlueprintHelperLibrary.GetBlackboard` (`AIBlueprintHelperLibrary.GetAIController` self)) "FanAttackLocation" (`SceneComponent.K2_GetComponentLocation` (`self.FanAttackLocation`))))))

(event `self.ReceiveBeginPlay`
  (`KismetSystemLibrary.K2_SetTimer` null "DigEffect" 0.01 true)
  (`self.DigUp`)
  (set `self.MaxHealth` (`self.Health`)))

(event `self.Death`
  (bind _returnvalue (`GameplayStatics.GetActorOfClass` "/Game/RoomMakerTools/BP_BossRoomManager2.BP_BossRoomManager2_C"))
  (`RoomManagerBase.SpawnLoot` _returnvalue))

(event `SpawnGoons`
  (for _array_element (`self.SpawnPositions`)
    (bind (_returnvalue_location _returnvalue_rotation) (`KismetMathLibrary.BreakTransform` (`SceneComponent.K2_GetComponentToWorld` _array_element)))
    (bind _returnvalue (`|SpawnActorFromClass` "/Game/Enemy/Cactucino/BP_Goon.BP_Goon_C" (`KismetMathLibrary.MakeTransform` _returnvalue_location _returnvalue_rotation) "Undefined" "MultiplyWithRoot" null self null))
    (`KismetArrayLibrary.Array_Add` (`self.Goons`) _returnvalue)))

(event `SpawnSpikeExplosion`
  (`|SpawnActorFromClass` "/Game/Enemy/Cactucino/BP_MafiaSpikeExplosion.BP_MafiaSpikeExplosion_C" (`self.GetTransform`) "Undefined" "MultiplyWithRoot" null null))

(event `BurstAttack`
  (`|SpawnActorFromClass` "/Game/Enemy/Cactucino/BP_MafiaProjectile.BP_MafiaProjectile_C" (`SceneComponent.K2_GetComponentToWorld` (`self.FiringLocation1`)) "Undefined" "MultiplyWithRoot" null 10.0 null))

(event `StartDigging`
  (if (not (`self.bIsDigging`))
    (bind (_direction _height) (`Timeline|Timeline_0` :!via `ReverseFromEnd`)
      (:`Update`
        (`SceneComponent.K2_SetRelativeLocation` (`self.Mesh`) (`KismetMathLibrary.MakeVector` 0.0 0.0 _height) false false))
      (:`Finished`
        (set `self.bIsDigging` true)))))

(event `FireCooldown`
  (set `self.Fire` true))

(event `FanAttack`
  (bind (_direction _rotation) (`Timeline|Timeline_2` :!via `PlayFromStart`)
    (:`Update`
      (`self.K2_SetActorRotation` (`KismetMathLibrary.MakeRotator` 0.0 0.0 _rotation))
      (if (`self.Fire`)
        (set `self.Fire` false)
        (for _array_element (`self.FiringLocations`)
          (`|SpawnActorFromClass` "/Game/Enemy/Cactucino/BP_MafiaProjectileSlow.BP_MafiaProjectileSlow_C" (`SceneComponent.K2_GetComponentToWorld` _array_element) "Undefined" "MultiplyWithRoot" null 10.0 null)
          (`KismetSystemLibrary.K2_SetTimer` null "FireCooldown" 0.05))))))

(event `StopDigging`
  (if (`self.bIsDigging`)
    (set `self.bIsDigging` false)
    (bind (_direction _height) (`Timeline|Timeline_1` :!via `PlayFromStart`)
      (:`Update`
        (`SceneComponent.K2_SetRelativeLocation` (`self.Mesh`) (`KismetMathLibrary.MakeVector` 0.0 0.0 _height) false false)))))

(event `FanAttackChargeUp`
  (bind (_direction _rotation) (`Timeline|Timeline_3` :!via `PlayFromStart`)
    (:`Update`
      (`self.K2_SetActorRotation` (`KismetMathLibrary.MakeRotator` 0.0 0.0 _rotation)))))

(event `self.BodyHitbox.OnComponentBeginOverlap`
  (params (OverlappedComponent :type "PrimitiveComponent Object Reference") (OtherActor :type "Actor Object Reference") (OtherComp :type "PrimitiveComponent Object Reference") (OtherBodyIndex :type Integer) (bFromSweep :type Boolean) (SweepResult :type "HitResult Structure (by ref)"))
  (bind (_returnvalue_x _returnvalue_y) (`KismetMathLibrary.BreakVector` (* (`KismetMathLibrary.Normal` (- (`self.K2_GetActorLocation`) (`self.K2_GetActorLocation`))) 400.0)))
  (if (not (`self.bIsDigging`))
    (bind _asplayer_character_base (cast `PlayerCharacterBase` OtherActor))
    (`GameplayStatics.ApplyDamage` _asplayer_character_base 20.0)
    (`self.LaunchCharacter` _asplayer_character_base (`KismetMathLibrary.MakeVector` _returnvalue_x _returnvalue_y 200.0) true true)))

(event `self.HeadHitbox.OnComponentBeginOverlap`
  (params (OverlappedComponent :type "PrimitiveComponent Object Reference") (OtherActor :type "Actor Object Reference") (OtherComp :type "PrimitiveComponent Object Reference") (OtherBodyIndex :type Integer) (bFromSweep :type Boolean) (SweepResult :type "HitResult Structure (by ref)"))
  (if (not (`self.bIsDigging`))
    (bind _asplayer_character_base (cast `PlayerCharacterBase` OtherActor))
    (`GameplayStatics.ApplyDamage` _asplayer_character_base 30.0)
    (`self.LaunchCharacter` _asplayer_character_base (0.0 0.0 600.0) true true)))

(event `DigEffect`
  (bind _returnvalue (`SceneComponent.K2_GetComponentToWorld` (`self.StaticMesh1`)))
  (if (`self.bIsDigging`)
    (`|SpawnActorFromClass` "/Game/Enemy/Cactucino/BP_DigEffect.BP_DigEffect_C" (`KismetMathLibrary.MakeTransform` (`KismetMathLibrary.MakeVector` (.x (.location _returnvalue)) (.y (.location _returnvalue)) (+ (.z (.location _returnvalue)) 30.0)) (.rotation _returnvalue) (.scale _returnvalue)) "Undefined" "MultiplyWithRoot" null null)))

(fn `MakeDynamicMaterial`
  (bind _mesh (`self.Mesh`))
  (for (_array_element _array_index) (`MeshComponent.GetMaterials` _mesh)
    (bind _returnvalue (`PrimitiveComponent.CreateDynamicMaterialInstance` _mesh _array_index _array_element "None"))
    (`PrimitiveComponent.SetMaterial` _mesh _array_index _returnvalue)
    (`KismetArrayLibrary.Array_Add` (`self.Dynamic Materials`) _returnvalue)))

(fn `UserConstructionScript`
  (bind _mesh (`self.Mesh`))
  (`|ExecutionSequence`
    (:`then_0`
      (set `self.SpawnPositions` (`|MakeArray` (`self.Goon1`) (`self.Goon2`) (`self.Goon3`) (`self.Goon4`))))
    (:`then_1`
      (for (_array_element _array_index) (`MeshComponent.GetMaterials` (`self.Mesh`))
        (bind _returnvalue (`PrimitiveComponent.CreateDynamicMaterialInstance` _mesh _array_index _array_element "None"))
        (`PrimitiveComponent.SetMaterial` _mesh _array_index _returnvalue)
        (`KismetArrayLibrary.Array_Add` (`self.Dynamic Materials`) _returnvalue)))
    (:`then_2`
      (set `self.FiringLocations` (`|MakeArray` (`self.FiringLocation4`) (`self.FiringLocation2`) (`self.FiringLocation3`) (`self.FiringLocation1`))))))