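; Royal Shroom bomber enemy character with two spawn modes: a bouncing launch and an upside-down ground-triggered bomb.
; NormalSpawn multicasts a bounce animation, hops forward after a random delay, rockets straight up, then destroys itself.
; SpecialSpawn multicasts a mesh Z-flip and starts a looping timer that line-traces downward, calling ServerExplode, which is defined outside these graphs, on a hit.
; The construction script creates and stores dynamic instances of the mesh materials.
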(event `MulticastAnim1`
  (`SkeletalMeshComponent.PlayAnimation` (`self.Mesh`) "/Game/Enemy/Mushroom/Rigs/MushroomBounceAnimRo__1_.MushroomBounceAnimRo__1_" false))

(event `NormalSpawn`
  (bind (_newvar_x _newvar_y) (`KismetMathLibrary.BreakVector` (`self.NewVar`)))
  (`self.MulticastAnim1`)
  (set `self.NewVar` (`self.GetActorForwardVector`))
  (`KismetSystemLibrary.Delay` (`KismetMathLibrary.RandomFloatInRange` 0.25 1.5))
  (`self.LaunchCharacter` (+ (* (`KismetMathLibrary.MakeVector` _newvar_x _newvar_y) 165.0) (0.0 0.0 900.0)))
  (`KismetSystemLibrary.Delay` 1.0)
  (set `MovementComponent.Velocity` (0.0 0.0 0.0) (`self.CharacterMovement`))
  (`self.LaunchCharacter` (0.0 0.0 3500.0))
  (`KismetSystemLibrary.Delay` 2.0)
  (`self.K2_DestroyActor`))

(event `MulticastSetScale`
  (`SceneComponent.SetWorldScale3D` (`self.Mesh`) (1.0 1.0 -1.0)))

(event `SpecialSpawn`
  (`self.MulticastSetScale`)
  (`KismetSystemLibrary.K2_SetTimer` null "CheckForGround" 0.06 true))

(event `CheckForGround`
  (bind _returnvalue (`self.K2_GetActorLocation`))
  (bind (_outhit _returnvalue_2) (`KismetSystemLibrary.LineTraceSingle` _returnvalue (- _returnvalue (0.0 0.0 150.0)) "TraceTypeQuery1"))
  (if _returnvalue_2
    (`self.Server_Explode`)
    (`KismetSystemLibrary.PrintString` "Hello")))

(fn `UserConstructionScript`
  (bind _mesh (`self.Mesh`))
  (for (_array_element _array_index) (`MeshComponent.GetMaterials` _mesh)
    (bind _returnvalue (`PrimitiveComponent.CreateDynamicMaterialInstance` _mesh _array_index _array_element "None"))
    (`PrimitiveComponent.SetMaterial` _mesh _array_index _returnvalue)
    (`KismetArrayLibrary.Array_Add` (`self.DynamicMaterials`) _returnvalue)))