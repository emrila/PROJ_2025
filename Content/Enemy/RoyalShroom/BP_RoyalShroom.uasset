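; Royal Shroom duo boss enemy: on the server, each links to its partner via blackboard and runs a behavior tree.
; At zero partner health both die, ending the fight; otherwise it goes down and flags the partner to revive it, respecting cooldown, with health refilling gradually.
; A tick-driven cooldown list toggles named attack flags, one gating overlap damage that multicasts a player squash.
; It also spawns bombers and flashes dynamic materials when hit.
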(event `self.ReceiveBeginPlay`
  (bind _returnvalue (`AIBlueprintHelperLibrary.GetAIController` self))
  (`/Engine/EditorBlueprintResources/ActorMacros.Switch Has Authority`
    (:`Authority`
      (`KismetSystemLibrary.Delay` 1.5)
      (bind _returnvalue_2 (`GameplayStatics.GetActorOfClass` "/Game/RoomMakerTools/BP_BossRoomManager.BP_BossRoomManager_C"))
      (set `self.BossManager` _returnvalue_2)
      (bind _outactors (`GameplayStatics.GetAllActorsOfClass` "BP_RoyalShroom_C"))
      (`AIController.UseBlackboard` _returnvalue "/Game/Enemy/RoyalShroom/BB_RoyalShroom.BB_RoyalShroom")
      (for _array_element _outactors
        (if (!= _array_element self)
          (`BlackboardComponent.SetValueAsObject` (`AIBlueprintHelperLibrary.GetBlackboard` _returnvalue) "DuoPartner" _array_element)
          (`KismetSystemLibrary.PrintString` "found")))
      (`KismetSystemLibrary.Delay` 4.0)
      (`AIController.RunBehaviorTree` _returnvalue "/Game/Enemy/RoyalShroom/BT_RoyalShroom.BT_RoyalShroom"))))

(event `ResetAttack`
  (params (CooldownName :type String) (CooldownTime :type "Float (double-precision)"))
  (bind _boolmap (`self.BoolMap`))
  (bind (_value _returnvalue) (`BlueprintMapLibrary.Map_Find` _boolmap CooldownName))
  (bind (_value_2 _returnvalue_2) (`BlueprintMapLibrary.Map_Find` _boolmap (`KismetStringLibrary.Mid` CooldownName 0 (- (`KismetStringLibrary.Len` CooldownName) 8))))
  (`KismetArrayLibrary.Array_Add` (`self.ActiveCooldowns`) (make `/Game/Enemy/RoyalShroom/RoyalCooldown` CooldownName CooldownTime))
  (if _returnvalue_2
    (`KismetArrayLibrary.Array_Set` (`self.Bools`) _value_2))
  (if _returnvalue
    (`KismetArrayLibrary.Array_Set` (`self.Bools`) _value true)))

(event `TickCooldowns`
  (for (_array_element _array_index) (`self.ActiveCooldowns`)
    (bind (_cooldownname _timer) (break `/Game/Enemy/RoyalShroom/RoyalCooldown` _array_element))
    (bind _structout (setmembers `/Game/Enemy/RoyalShroom/RoyalCooldown` :`StructRef` _array_element :`CooldownName` _cooldownname :`Timer` (- _timer (`GameplayStatics.GetWorldDeltaSeconds`))))
    (`KismetArrayLibrary.Array_Set` (`self.ActiveCooldowns`) _array_index _structout)
    (bind (_output_cooldownname _output_timer) (break `/Game/Enemy/RoyalShroom/RoyalCooldown` (`|GetArrayItem` (`self.ActiveCooldowns`) _array_index)))
    (if (<= _output_timer 0.0)
      (`KismetArrayLibrary.Array_Set` (`self.Bools`) (`BlueprintMapLibrary.Map_Find` (`self.BoolMap`) _output_cooldownname))
      (`KismetArrayLibrary.Array_Remove` (`self.ActiveCooldowns`) _array_index))))

(event `self.CheckForDeath`
  (bind _asbp_royal_shroom (cast `/Game/Enemy/RoyalShroom/BP_RoyalShroom` (`BlackboardComponent.GetValueAsObject` (`AIBlueprintHelperLibrary.GetBlackboard` (`AIBlueprintHelperLibrary.GetAIController` self)) "DuoPartner")))
  (if (<= (`EnemyBase.Health` _asbp_royal_shroom) 0.0)
    (`self.FinishBoss`)
    (`self.SuperDestroy` _asbp_royal_shroom)
    (`self.SuperDestroy`)
    (else
      (`BlackboardComponent.SetValueAsBool` (`AIBlueprintHelperLibrary.GetBlackboard` (`AIBlueprintHelperLibrary.GetAIController` self)) "IsDowned" true)
      (set `self.IsCurrentlyDowned` true)
      (set `self.ReviveDelayed` false)
      (for _array_element (`self.ActiveCooldowns`)
        (if (and (`KismetStringLibrary.EqualEqual_StrStr` (break `/Game/Enemy/RoyalShroom/RoyalCooldown` _array_element) "ReviveCooldown") (> (`.Timer_5_7ED9AC184B212D6AE9057989F1CFE863` (break `/Game/Enemy/RoyalShroom/RoyalCooldown` _array_element)) 0.0))
          (`KismetSystemLibrary.K2_SetTimer` null "RevivePartnerDelayed" (`.Timer_5_7ED9AC184B212D6AE9057989F1CFE863` (break `/Game/Enemy/RoyalShroom/RoyalCooldown` _array_element)))
          (set `self.ReviveDelayed` true)
          (break)))
      (if (not (`self.ReviveDelayed`))
        (`BlackboardComponent.SetValueAsBool` (`AIBlueprintHelperLibrary.GetBlackboard` (`AIBlueprintHelperLibrary.GetAIController` _asbp_royal_shroom)) "Revive" true)))))

(event `self.ReceiveTick`
  (params (DeltaSeconds :type "Float (single-precision)"))
  (`self.TickCooldowns`))

(event `SpawnBomberAt`
  (params (Location :type "Vector Structure") (SpecialSpawn :type Boolean))
  (bind _returnvalue (`|SpawnActorFromClass` "/Game/Enemy/RoyalShroom/BP_RoyaShroomlBomber.BP_RoyaShroomlBomber_C" (`KismetMathLibrary.MakeTransform` Location (`KismetMathLibrary.FindLookAtRotation` Location (`self.K2_GetActorLocation`))) "Undefined" "MultiplyWithRoot" null null))
  (set `EnemyBase.DamageMultiplier` 2.0 _returnvalue)
  (if SpecialSpawn
    (`/Game/Enemy/RoyalShroom/BP_RoyaShroomlBomber.SpecialSpawn` _returnvalue)
    (else
      (`/Game/Enemy/RoyalShroom/BP_RoyaShroomlBomber.NormalSpawn` _returnvalue))))

(event `self.Sphere.OnComponentBeginOverlap`
  (params (OverlappedComponent :type "PrimitiveComponent Object Reference") (OtherActor :type "Actor Object Reference") (OtherComp :type "PrimitiveComponent Object Reference") (OtherBodyIndex :type Integer) (bFromSweep :type Boolean) (SweepResult :type "HitResult Structure (by ref)"))
  (`/Engine/EditorBlueprintResources/ActorMacros.Switch Has Authority`
    (:`Authority`
      (if (`|GetArrayItem` (`self.Bools`))
        (bind _asbp_player_character_base (cast `/Game/Developer/Basir/BP_PlayerCharacterBase` OtherActor))
        (`GameplayStatics.ApplyDamage` _asbp_player_character_base 20.0)
        (`self.MulticastPlayerScale` _asbp_player_character_base)))))

(event `RevivePartnerDelayed`
  (bind _asbp_royal_shroom (cast `/Game/Enemy/RoyalShroom/BP_RoyalShroom` (`BlackboardComponent.GetValueAsObject` (`AIBlueprintHelperLibrary.GetBlackboard` (`AIBlueprintHelperLibrary.GetAIController` self)) "DuoPartner")))
  (`BlackboardComponent.SetValueAsBool` (`AIBlueprintHelperLibrary.GetBlackboard` (`AIBlueprintHelperLibrary.GetAIController` _asbp_royal_shroom)) "Revive" true))

(event `Reivive`
  (params (ReviveHealth :type "Float (double-precision)"))
  (set `self.RestoredHealth` 0.0)
  (set `self.TargetHealth` ReviveHealth)
  (`KismetSystemLibrary.K2_SetTimer` null "RestoreHealth" 0.01)
  (`KismetSystemLibrary.Delay` 5.0)
  (`BlackboardComponent.SetValueAsBool` (`AIBlueprintHelperLibrary.GetBlackboard` (`AIBlueprintHelperLibrary.GetAIController` self)) "IsDowned" false))

(event `MulticastPlayerScale`
  (params (PlayerToSquish :type "/Game/Developer/Basir/BP_PlayerCharacterBase Object Reference"))
  (bind _mesh (`Character.Mesh` PlayerToSquish))
  (`SceneComponent.SetWorldScale3D` _mesh (1.0 1.0 0.1))
  (bind (_direction _newtrack_0) (`Timeline|Timeline` :!via `PlayFromStart`)
    (:`Update`
      (`SceneComponent.SetWorldScale3D` _mesh (`KismetMathLibrary.MakeVector` 1.0 1.0 _newtrack_0)))))

(event `RestoreHealth`
  (set `self.Health` (+ (`self.Health`) (/ (`self.TargetHealth`) 200.0)))
  (set `self.RestoredHealth` (+ (`self.RestoredHealth`) (/ (`self.TargetHealth`) 200.0)))
  (`self.RefreshHPBar`)
  (if (>= (`self.RestoredHealth`) (`self.TargetHealth`))
    (set `self.IsCurrentlyDowned` false)
    (else
      (`KismetSystemLibrary.K2_SetTimer` null "RestoreHealth" 0.01))))

(event `self.HitFeedback`
  (for _array_element (`self.DynamicMaterials`)
    (`MaterialInstanceDynamic.SetScalarParameterValue` _array_element "DamageToggle" 1.0))
  (`KismetSystemLibrary.Delay` 0.1)
  (for _array_element_2 (`self.DynamicMaterials`)
    (`MaterialInstanceDynamic.SetScalarParameterValue` _array_element_2 "DamageToggle" 0.0)))

(fn `UserConstructionScript`
  (bind _mesh (`self.Mesh`))
  (for (_array_element _array_index) (`MeshComponent.GetMaterials` _mesh)
    (bind _returnvalue (`PrimitiveComponent.CreateDynamicMaterialInstance` _mesh _array_index _array_element "None"))
    (`PrimitiveComponent.SetMaterial` _mesh _array_index _returnvalue)
    (`KismetArrayLibrary.Array_Add` (`self.DynamicMaterials`) _returnvalue)))