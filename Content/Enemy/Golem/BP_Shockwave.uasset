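; Golem enemy shockwave actor that spreads outward as a growing ring and punishes players who stay on the ground.
; A looping timer steadily widens the static mesh on X and Y while keeping Z fixed, and the actor destroys itself after a short delay.
; Mesh overlap damages a player character only if it is moving on the ground, then launches it upward, so airborne players avoid the hit.
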(event `self.ReceiveBeginPlay`
  (`KismetSystemLibrary.K2_SetTimer` null "Expand" 0.01 true)
  (`KismetSystemLibrary.Delay` 5.0)
  (`self.K2_DestroyActor`))

(event `Expand`
  (bind _staticmesh (`self.StaticMesh`))
  (bind (_returnvalue_x _returnvalue_y) (`KismetMathLibrary.BreakVector` (`SceneComponent.K2_GetComponentScale` _staticmesh)))
  (`SceneComponent.SetWorldScale3D` _staticmesh (`KismetMathLibrary.MakeVector` (+ _returnvalue_x 0.1) (+ _returnvalue_y 0.1) 1.0)))

(event `self.StaticMesh.OnComponentBeginOverlap`
  (params (OverlappedComponent :type "PrimitiveComponent Object Reference") (OtherActor :type "Actor Object Reference") (OtherComp :type "PrimitiveComponent Object Reference") (OtherBodyIndex :type Integer) (bFromSweep :type Boolean) (SweepResult :type "HitResult Structure (by ref)"))
  (bind _asplayer_character_base (cast `PlayerCharacterBase` OtherActor))
  (if (`NavMovementComponent.IsMovingOnGround` (`Character.CharacterMovement` _asplayer_character_base))
    (`GameplayStatics.ApplyDamage` _asplayer_character_base (* (`self.Base Damage`) (`self.DamageMultiplier`)))
    (`Character.LaunchCharacter` _asplayer_character_base (0.0 0.0 500.0) false false)))

(fn `UserConstructionScript`)