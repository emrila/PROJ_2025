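; BP_GolemBeam is a golem beam attack actor, pairing a sphere with a child BP_Beam that receives its damage value and a placeholder head material.
; On BeginPlay, a timeline drives the sphere's height and yaw, with events that disable sphere collision and remove the beam.
; The actor destroys itself when the timeline finishes.
; If the golem's health runs out first, the beam is removed and the sphere becomes a physics object before delayed destruction.
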(event `self.ReceiveBeginPlay`
  (bind _sphere (`self.Sphere`))
  (bind _childactor (`self.ChildActor`))
  (bind _childactor_2 (`self.ChildActor`))
  (bind (_relativerotation_roll _relativerotation_pitch) (`KismetMathLibrary.BreakRotator` (`SceneComponent.RelativeRotation` _sphere)))
  (bind (_relativelocation_x _relativelocation_y) (`KismetMathLibrary.BreakVector` (`SceneComponent.RelativeLocation` _sphere)))
  (bind _asbp_beam (cast `/Game/Obstacles/BP_Beam` (`ChildActorComponent.ChildActor` (`self.ChildActor`))))
  (set `/Game/Obstacles/BP_Beam.Damage` (`self.Damage`) _asbp_beam)
  (bind (_direction _height _rotation) (`Timeline|AttackTimeline` :!via `PlayFromStart` :!label _label)
    (:`Update`
      (if (> (`EnemyBase.Health` (`self.Golem`)) 0.0)
        (`SceneComponent.K2_SetRelativeRotation` _sphere (`KismetMathLibrary.MakeRotator` _relativerotation_roll _relativerotation_pitch _rotation) false false)
        (`SceneComponent.K2_SetRelativeLocation` _sphere (`KismetMathLibrary.MakeVector` _relativelocation_x _relativelocation_y _height) false false)
        (else
          (`/Engine/EditorBlueprintResources/StandardMacros.IsValid` _childactor
            (:`Is Valid`
              (`ActorComponent.K2_DestroyComponent` _childactor)
              (`PrimitiveComponent.SetSimulatePhysics` (`self.Sphere`) true)
              (`PrimitiveComponent.SetCollisionEnabled` (`self.Sphere`) "QueryAndPhysics")
              (`|ExecutionSequence`
                (:`then_0`
                  (goto _label :!via `Stop`))
                (:`then_1`
                  (`KismetSystemLibrary.Delay` 5.0)
                  (`self.K2_DestroyActor`))))))))
    (:`Finished`
      (if (> (`EnemyBase.Health` (`self.Golem`)) 0.0)
        (`self.K2_DestroyActor`)))
    (:`StartLaser`
      (`PrimitiveComponent.SetCollisionEnabled` (`self.Sphere`) "NoCollision"))
    (:`DestroyBeam`
      (`/Engine/EditorBlueprintResources/StandardMacros.IsValid` _childactor_2
        (:`Is Valid`
          (`ActorComponent.K2_DestroyComponent` _childactor_2))))))

(fn `UserConstructionScript`
  (bind _asbp_beam (cast `/Game/Obstacles/BP_Beam` (`ChildActorComponent.ChildActor` (`self.ChildActor`))))
  (`/Game/Obstacles/BP_Beam.SetMaterial` _asbp_beam "/Game/Enemy/Golem/Materials/M_PlaceholderGolemHead.M_PlaceholderGolemHead"))