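; Golem enemy character that damages and knocks back players with a charge and a melee combo ending in a ground slam.
; Melee chains into MeleeFollowup and Groundslam through Delays, animating the attacks by rotating and offsetting arm components, then spawning BP_Shockwave at the right arm.
; Capsule and arm hitbox overlaps only hit while their state flags are set.
; Charging is only read here, and SetSpeed exposes walk speed changes.
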(event `self.ReceiveBeginPlay`)

(event `self.CapsuleComponent.OnComponentBeginOverlap`
  (params (OverlappedComponent :type "PrimitiveComponent Object Reference") (OtherActor :type "Actor Object Reference") (OtherComp :type "PrimitiveComponent Object Reference") (OtherBodyIndex :type Integer) (bFromSweep :type Boolean) (SweepResult :type "HitResult Structure (by ref)"))
  (if (`self.Charging`)
    (bind _asplayer_character_base (cast `PlayerCharacterBase` OtherActor))
    (`GameplayStatics.ApplyDamage` _asplayer_character_base 40.0 null null "/Script/Engine.DamageType")
    (`self.LaunchCharacter` _asplayer_character_base (* (`self.GetActorForwardVector`) 2000.0) false false)
    (`MovementComponent.StopMovementImmediately` (`self.CharacterMovement`))))

(event `Melee`
  (set `self.RMelee` true)
  (`SceneComponent.K2_AddWorldRotation` (`self.RightArm`) (struct :`Yaw` 90.0) false false)
  (`KismetSystemLibrary.Delay` 0.5)
  (set `self.RMelee` false)
  (`KismetSystemLibrary.Delay` 0.5)
  (`self.MeleeFollowup`))

(event `self.RMeleeHitbox.OnComponentBeginOverlap`
  (params (OverlappedComponent :type "PrimitiveComponent Object Reference") (OtherActor :type "Actor Object Reference") (OtherComp :type "PrimitiveComponent Object Reference") (OtherBodyIndex :type Integer) (bFromSweep :type Boolean) (SweepResult :type "HitResult Structure (by ref)"))
  (if (`self.RMelee`)
    (bind _asplayer_character_base (cast `PlayerCharacterBase` OtherActor))
    (`GameplayStatics.ApplyDamage` _asplayer_character_base 50.0 null null "/Script/Engine.DamageType")
    (`self.LaunchCharacter` _asplayer_character_base (* (`self.GetActorForwardVector`) 1000.0) false false)
    (set `self.RMelee` false)))

(event `MeleeFollowup`
  (set `self.LMelee` true)
  (`SceneComponent.K2_AddWorldRotation` (`self.RightArm`) (struct :`Yaw` -90.0) false false)
  (`KismetSystemLibrary.Delay` 1.0)
  (`SceneComponent.K2_AddWorldRotation` (`self.LeftArm`) (struct :`Yaw` -90.0) false false)
  (`KismetSystemLibrary.Delay` 0.5)
  (set `self.LMelee` false)
  (`KismetSystemLibrary.Delay` 0.5)
  (`SceneComponent.K2_AddWorldRotation` (`self.LeftArm`) (struct :`Yaw` 90.0) false false)
  (`self.Groundslam`))

(event `self.LMeleeHitbox.OnComponentBeginOverlap`
  (params (OverlappedComponent :type "PrimitiveComponent Object Reference") (OtherActor :type "Actor Object Reference") (OtherComp :type "PrimitiveComponent Object Reference") (OtherBodyIndex :type Integer) (bFromSweep :type Boolean) (SweepResult :type "HitResult Structure (by ref)"))
  (if (`self.LMelee`)
    (bind _asplayer_character_base (cast `PlayerCharacterBase` OtherActor))
    (`GameplayStatics.ApplyDamage` _asplayer_character_base 50.0 null null "/Script/Engine.DamageType")
    (`self.LaunchCharacter` _asplayer_character_base (* (`self.GetActorForwardVector`) 1000.0) false false)
    (set `self.LMelee` false)))

(event `Groundslam`
  (bind _rightarm (`self.RightArm`))
  (`KismetSystemLibrary.Delay` 1.0)
  (set `self.Slam` true)
  (`SceneComponent.K2_AddWorldOffset` (`self.RightArm`) (0.0 0.0 80.0) false false)
  (`SceneComponent.K2_AddWorldOffset` (`self.LeftArm`) (0.0 0.0 80.0) false false)
  (`KismetSystemLibrary.Delay` 1.0)
  (`SceneComponent.K2_AddWorldOffset` _rightarm (0.0 0.0 -160.0) false false)
  (`SceneComponent.K2_AddWorldOffset` (`self.LeftArm`) (0.0 0.0 -160.0) false false)
  (`|SpawnActorFromClass` "/Game/Enemy/Golem/BP_Shockwave.BP_Shockwave_C" (`KismetMathLibrary.MakeTransform` (`SceneComponent.K2_GetComponentLocation` _rightarm)) "Undefined" "MultiplyWithRoot" null null)
  (`KismetSystemLibrary.Delay` 1.0)
  (`SceneComponent.K2_AddWorldOffset` (`self.RightArm`) (0.0 0.0 80.0) false false)
  (`SceneComponent.K2_AddWorldOffset` (`self.LeftArm`) (0.0 0.0 80.0) false false))

(event `SetSpeed`
  (params (Speed :type "Float (double-precision)"))
  (set `CharacterMovementComponent.MaxWalkSpeed` Speed (`self.CharacterMovement`)))

(fn `UserConstructionScript`)