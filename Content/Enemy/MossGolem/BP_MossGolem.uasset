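; Moss Golem enemy character with melee swings, a ground slam, a forward leap and a charge, roaring on spawn.
; Start/End melee events resize per-hand hitbox spheres, whose player overlaps trace to apply damage and knockback.
; Slam traces down between both hands to spawn a shockwave.
; Capsule hits while charging damage and fling characters, while other obstacles stun the golem via Blackboard; death stops AI logic.
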(event `self.ReceiveBeginPlay`
  (set `self.MaxHealth` (`self.Health`))
  (`self.PlayAnimation` "/Game/Enemy/MossGolem/Animation/Montages/AM_Roar.AM_Roar"))

(event `Slam`
  (bind (_returnvalue_x _returnvalue_y _returnvalue_z) (`KismetMathLibrary.BreakVector` (`SceneComponent.K2_GetComponentLocation` (`self.Mesh`))))
  (bind _returnvalue (/ (+ (`SceneComponent.K2_GetComponentLocation` (`self.LeftMeleeHitbox`)) (`SceneComponent.K2_GetComponentLocation` (`self.RightMeleeHitbox`))) 2))
  (bind _outhit (`KismetSystemLibrary.LineTraceSingle` (+ _returnvalue (0.0 0.0 10.0)) (- _returnvalue (0.0 0.0 100.0)) "TraceTypeQuery1" false (`|MakeArray` self :!type "Actor Object Reference") "ForDuration"))
  (bind (_bblockinghit _binitialoverlap _time _distance _location _impactpoint) (`GameplayStatics.BreakHitResult` _outhit))
  (if _bblockinghit
    (`|SpawnActorFromClass` "/Game/Enemy/MossGolem/BP_Shockwave.BP_Shockwave_C" (`KismetMathLibrary.MakeTransform` (`KismetMathLibrary.MakeVector` (.x _impactpoint) (.y _impactpoint) _returnvalue_z)) "Undefined" "MultiplyWithRoot" null null)))

(event `Leap`
  (bind (_returnvalue_x _returnvalue_y) (`KismetMathLibrary.BreakVector` (* (`self.GetActorForwardVector`) 500.0)))
  (set `self.bCharging` false)
  (`self.LaunchCharacter` (`KismetMathLibrary.MakeVector` _returnvalue_x _returnvalue_y 600.0) true true))

(event `self.RightMeleeHitbox.OnComponentBeginOverlap`
  (params (OverlappedComponent :type "PrimitiveComponent Object Reference") (OtherActor :type "Actor Object Reference") (OtherComp :type "PrimitiveComponent Object Reference") (OtherBodyIndex :type Integer) (bFromSweep :type Boolean) (SweepResult :type "HitResult Structure (by ref)"))
  (if (`self.bRightMelee`)
    (`self.DealMeleeDamage` OtherActor (`self.RightMeleeHitbox`))))

(event `SetSpeed`
  (params (Speed :type "Float (double-precision)"))
  (set `CharacterMovementComponent.MaxWalkSpeed` Speed (`self.CharacterMovement`)))

(event `self.LeftMeleeHitbox.OnComponentBeginOverlap`
  (params (OverlappedComponent :type "PrimitiveComponent Object Reference") (OtherActor :type "Actor Object Reference") (OtherComp :type "PrimitiveComponent Object Reference") (OtherBodyIndex :type Integer) (bFromSweep :type Boolean) (SweepResult :type "HitResult Structure (by ref)"))
  (if (`self.bLeftMelee`)
    (`self.DealMeleeDamage` OtherActor (`self.LeftMeleeHitbox`))))

(event `StartLeftMelee`
  (set `self.bLeftMelee` true)
  (`SphereComponent.SetSphereRadius` (`self.LeftMeleeHitbox`) 50.0 true))

(event `EndLeftMelee`
  (set `self.bLeftMelee` false)
  (`SphereComponent.SetSphereRadius` (`self.LeftMeleeHitbox`) 1.0 true))

(event `StartRightMelee`
  (set `self.bRightMelee` true)
  (`SphereComponent.SetSphereRadius` (`self.RightMeleeHitbox`) 50.0 true))

(event `EndRightMelee`
  (set `self.bRightMelee` false)
  (`SphereComponent.SetSphereRadius` (`self.RightMeleeHitbox`) 1.0 true))

(event `PlayAnimation`
  (params (AnimMontage :type "AnimMontage Object Reference"))
  (`|PlayMontage` (`self.Mesh`) AnimMontage))

(event `self.CapsuleComponent.OnComponentHit`
  (params (HitComponent :type "PrimitiveComponent Object Reference") (OtherActor :type "Actor Object Reference") (OtherComp :type "PrimitiveComponent Object Reference") (NormalImpulse :type "Vector Structure") (Hit :type "HitResult Structure (by ref)"))
  (bind (_returnvalue_x _returnvalue_y) (`KismetMathLibrary.BreakVector` (* (`KismetMathLibrary.RandomUnitVectorInConeInDegrees` (`self.GetActorForwardVector`) 100.0) 2000.0)))
  (if (`self.bCharging`)
    (`GameplayStatics.ApplyDamage` OtherActor (* (`self.ChargeDamage`) (`self.DamageMultiplier`)))
    (bind _ascharacter (cast `Character` OtherActor)
      (:`then`
        (`self.LaunchCharacter` _ascharacter (`KismetMathLibrary.MakeVector` _returnvalue_x _returnvalue_y 100.0) true true))
      (:`CastFailed`
        (`MovementComponent.StopMovementImmediately` (`self.CharacterMovement`))
        (set `self.bStunned` true)
        (`BlackboardComponent.SetValueAsBool` (`AIBlueprintHelperLibrary.GetBlackboard` null) "Stunned" true)))))

(event `self.OnRep_Death`
  (bind _returnvalue (`AIBlueprintHelperLibrary.GetAIController` self))
  (`/Engine/EditorBlueprintResources/StandardMacros.IsValid` _returnvalue :!label _label
    (:`Is Valid`
      (`BrainComponent.StopLogic` (`AIController.BrainComponent` _returnvalue) ""))
    (:`Is Not Valid`
      (`KismetSystemLibrary.RetriggerableDelay` 0.2)
      (goto _label))))

(event `self.HitFeedback`
  (`|PlayMontage` (`self.Mesh`) (`KismetArrayLibrary.Array_Random` (`self.HitAnimations`)) 2.0 0.0 "None" false))

(fn `DealMeleeDamage`
  (params (HitActor :type "Actor Object Reference") (Hitbox :type "SceneComponent Object Reference"))
  (bind (_returnvalue_x _returnvalue_y) (`KismetMathLibrary.BreakVector` (* (`self.GetActorForwardVector`) 500.0)))
  (cast `/Game/Developer/Basir/BP_PlayerCharacterBase` HitActor)
  (bind _outhit (`KismetSystemLibrary.LineTraceSingle` (`SceneComponent.K2_GetComponentLocation` Hitbox) (`self.K2_GetActorLocation` HitActor) "TraceTypeQuery1" false (`|MakeArray` self :!type "Actor Object Reference") "ForDuration"))
  (bind (_bblockinghit _binitialoverlap _time _distance _location _impactpoint _normal _impactnormal _physmat _hitactor) (`GameplayStatics.BreakHitResult` _outhit))
  (`GameplayStatics.ApplyDamage` _hitactor (* (`self.MeleeDamage`) (`self.DamageMultiplier`)))
  (bind _asbp_player_character_base (cast `/Game/Developer/Basir/BP_PlayerCharacterBase` _hitactor))
  (if (`self.bLeftMelee`)
    (bind (_returnvalue_x_2 _returnvalue_y_2) (`KismetMathLibrary.BreakVector` (* (- _impactpoint (`self.K2_GetActorLocation` _hitactor)) -25.0)))
    (`self.LaunchCharacter` _asbp_player_character_base (`KismetMathLibrary.MakeVector` _returnvalue_x_2 _returnvalue_y_2 200.0) true true)
    (else
      (`self.LaunchCharacter` _asbp_player_character_base (`KismetMathLibrary.MakeVector` _returnvalue_x _returnvalue_y 200.0) true true))))

(fn `UserConstructionScript`)