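; Moss Golem slam shockwave that plays the GolemSlam audio event, then expands outward for five seconds before destroying itself.
; A looping timer widens the sphere in X and Y, keeping its height fixed.
; On overlap, grounded players not below the wave's origin take scaled damage and are launched upward.
; Every overlapped player is recorded, so anyone airborne or below at first contact also avoids later hits.
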(event `self.ReceiveBeginPlay`
  (`FMODBlueprintStatics.PlayEventAttached` "/Game/FMOD/Events/Enemies/Golem/GolemSlam.GolemSlam" (`self.Sphere`) "None" (0.0 0.0 0.0) "KeepRelativeOffset")
  (`KismetSystemLibrary.K2_SetTimer` null "Expand" 0.01 true)
  (`KismetSystemLibrary.Delay` 5.0)
  (`self.K2_DestroyActor`))

(event `Expand`
  (bind _sphere (`self.Sphere`))
  (bind (_returnvalue_x _returnvalue_y) (`KismetMathLibrary.BreakVector` (`SceneComponent.K2_GetComponentScale` _sphere)))
  (`SceneComponent.SetWorldScale3D` _sphere (`KismetMathLibrary.MakeVector` (+ _returnvalue_x 0.071) (+ _returnvalue_y 0.071) 1.0)))

(event `self.Sphere.OnComponentBeginOverlap`
  (params (OverlappedComponent :type "PrimitiveComponent Object Reference") (OtherActor :type "Actor Object Reference") (OtherComp :type "PrimitiveComponent Object Reference") (OtherBodyIndex :type Integer) (bFromSweep :type Boolean) (SweepResult :type "HitResult Structure (by ref)"))
  (bind (_returnvalue_x _returnvalue_y _returnvalue_z) (`KismetMathLibrary.BreakVector` (`self.K2_GetActorLocation`)))
  (bind _asplayer_character_base (cast `PlayerCharacterBase` OtherActor))
  (bind (_returnvalue_x_2 _returnvalue_y_2 _returnvalue_z_2) (`KismetMathLibrary.BreakVector` (`self.K2_GetActorLocation` _asplayer_character_base)))
  (if (and (`NavMovementComponent.IsMovingOnGround` (`Character.CharacterMovement` _asplayer_character_base)) (not (> _returnvalue_z _returnvalue_z_2)))
    (if (not (`KismetArrayLibrary.Array_Contains` (`self.HasOverlapped`) _asplayer_character_base))
      (`GameplayStatics.ApplyDamage` _asplayer_character_base (* (`self.Base Damage`) (`self.DamageMultiplier`)))
      (`Character.LaunchCharacter` _asplayer_character_base (0.0 0.0 500.0) true true)
      (`KismetArrayLibrary.Array_Add` (`self.HasOverlapped`) _asplayer_character_base :!label _label))
    (else
      (goto _label))))

(fn `UserConstructionScript`)