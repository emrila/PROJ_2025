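; RoTaShroom mushroom enemy that hurts and knocks back the player on capsule contact.
; When AttackIsOnCooldown or Projectile is true, an overlapping player character takes multiplier-scaled damage and is launched along the enemy's forward vector with an upward lift.
; The construction script swaps every mesh material for a dynamic instance, which HitFeedback uses to briefly flash the DamageToggle parameter.
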(event `self.ReceiveBeginPlay`)

(event `self.CapsuleComponent.OnComponentBeginOverlap`
  (params (OverlappedComponent :type "PrimitiveComponent Object Reference") (OtherActor :type "Actor Object Reference") (OtherComp :type "PrimitiveComponent Object Reference") (OtherBodyIndex :type Integer) (bFromSweep :type Boolean) (SweepResult :type "HitResult Structure (by ref)"))
  (bind (_returnvalue_x _returnvalue_y) (`KismetMathLibrary.BreakVector` (* (`self.GetActorForwardVector`) 850.0)))
  (if (or (`self.AttackIsOnCooldown`) (`self.Projectile`))
    (bind _asplayer_character_base (cast `PlayerCharacterBase` OtherActor))
    (`GameplayStatics.ApplyDamage` _asplayer_character_base (* (`self.Base Damage`) (`self.DamageMultiplier`)) null null "/Script/Engine.DamageType")
    (`self.LaunchCharacter` _asplayer_character_base (`KismetMathLibrary.MakeVector` _returnvalue_x _returnvalue_y 180.0) false false)))

(event `self.HitFeedback`
  (for _array_element (`self.DynamicMaterials`)
    (`MaterialInstanceDynamic.SetScalarParameterValue` _array_element "DamageToggle" 1.0))
  (`KismetSystemLibrary.Delay` 0.1)
  (for _array_element_2 (`self.DynamicMaterials`)
    (`MaterialInstanceDynamic.SetScalarParameterValue` _array_element_2 "DamageToggle" 0.0)))

(fn `UserConstructionScript`
  (bind _mesh (`self.Mesh`))
  (for (_array_element _array_index) (`MeshComponent.GetMaterials` _mesh)
    (bind _returnvalue (`PrimitiveComponent.CreateDynamicMaterialInstance` _mesh _array_index _array_element "None"))
    (`PrimitiveComponent.SetMaterial` _mesh _array_index _returnvalue)
    (`KismetArrayLibrary.Array_Add` (`self.DynamicMaterials`) _returnvalue)))