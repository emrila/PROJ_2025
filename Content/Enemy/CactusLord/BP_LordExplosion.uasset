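; BP_LordExplosion is a short-lived Cactus Lord explosion that damages actors and knocks players back.
; On BeginPlay it plays the CactieBoom sound event, scales its Sphere through a timeline, then destroys itself.
; Overlaps trigger a debug-drawn visibility trace from the center, ignoring the Spawner, so blockers take the hit instead.
; Each traced actor is damaged once via HitActors, and player characters are launched outward and upward.
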(event `self.ReceiveBeginPlay`
  (bind _sphere (`self.Sphere`))
  (`FMODBlueprintStatics.PlayEventAttached` "/Game/FMOD/Events/Enemies/CactieBoom.CactieBoom" _sphere "None" (0.0 0.0 0.0) "KeepRelativeOffset")
  (bind (_direction _newtrack_0) (`Timeline|Timeline` :!via `PlayFromStart`)
    (:`Update`
      (`SceneComponent.SetWorldScale3D` _sphere (`KismetMathLibrary.Conv_DoubleToVector` _newtrack_0)))
    (:`Finished`
      (`self.K2_DestroyActor`))))

(event `self.ReceiveActorBeginOverlap`
  (params (OtherActor :type "Actor Object Reference"))
  (bind _outhit (`KismetSystemLibrary.LineTraceSingle` (`self.K2_GetActorLocation`) (`self.K2_GetActorLocation` OtherActor) "TraceTypeQuery1" false (`|MakeArray` (`self.Spawner`)) "ForDuration"))
  (bind (_bblockinghit _binitialoverlap _time _distance _location _impactpoint _normal _impactnormal _physmat _hitactor) (`GameplayStatics.BreakHitResult` _outhit))
  (if (not (`KismetArrayLibrary.Array_Contains` (`self.HitActors`) _hitactor))
    (`GameplayStatics.ApplyDamage` _hitactor (* (`self.DamageMultiplier`) (`self.Base Damage`)))
    (`KismetArrayLibrary.Array_Add` (`self.HitActors`) _hitactor)
    (bind _asbp_player_character_base (cast `/Game/Developer/Basir/BP_PlayerCharacterBase` _hitactor))
    (bind (_returnvalue_x _returnvalue_y) (`KismetMathLibrary.BreakVector` (* (`KismetMathLibrary.Normal` (- (`self.K2_GetActorLocation` _hitactor) (`self.K2_GetActorLocation`))) 200.0)))
    (`Character.LaunchCharacter` _asbp_player_character_base (`KismetMathLibrary.MakeVector` _returnvalue_x _returnvalue_y 200.0) true true)))

(fn `UserConstructionScript`)