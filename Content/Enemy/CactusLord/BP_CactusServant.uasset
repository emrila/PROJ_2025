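; BP_CactusServant is an enemy goon of the Cactus Lord boss that rises from below when it spawns.
; On BeginPlay it runs DigUp, dropping its mesh below its origin and animating the height with the Dig timeline, then sets its damage multiplier.
; On Death with no health left, it removes itself from the boss's Goons list and prints a debug message.
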(event `self.ReceiveBeginPlay`
  (`self.DigUp`)
  (set `self.DamageMultiplier` 2.0))

(event `self.Death`
  (if (<= (`self.Health`) 0.0)
    (`KismetArrayLibrary.Array_RemoveItem` (`/Game/Enemy/CactusLord/BP_CactusLord.Goons` (`self.Boss`)) self)
    (`KismetSystemLibrary.PrintString` "Goon Removed")))

(event `DigUp`
  (`SceneComponent.K2_SetRelativeLocation` (`self.StaticMesh`) (0.0 0.0 -180.0) false false)
  (bind (_direction _height) (`Timeline|Dig` :!via `PlayFromStart`)
    (:`Update`
      (`SceneComponent.K2_SetRelativeLocation` (`self.StaticMesh`) (`KismetMathLibrary.MakeVector` 0.0 0.0 _height) false false))))

(fn `UserConstructionScript`
  (`parent.UserConstructionScript`))