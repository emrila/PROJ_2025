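; BP_HealthPickup is a single-use pickup that restores health when a player character overlaps its sphere.
; The overlap is handled only with authority and calls Heal, which reveals the Niagara effect hidden at BeginPlay.
; Heal passes RestoreAmount to RestoreHealth on BP_WizardGameState, leaving the passed character unused.
; The FurkansBool flag then blocks further heals, while the actor stays in the world.
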(event `self.ReceiveBeginPlay`
  (set `self.FurkansBool` false)
  (`SceneComponent.SetHiddenInGame` (`self.Niagara`) true false))

(event `self.Sphere.OnComponentBeginOverlap`
  (params (OverlappedComponent :type "PrimitiveComponent Object Reference") (OtherActor :type "Actor Object Reference") (OtherComp :type "PrimitiveComponent Object Reference") (OtherBodyIndex :type Integer) (bFromSweep :type Boolean) (SweepResult :type "HitResult Structure (by ref)"))
  (`/Engine/EditorBlueprintResources/ActorMacros.Switch Has Authority`
    (:`Authority`
      (bind _asplayer_character_base (cast `PlayerCharacterBase` OtherActor))
      (if (not (`self.FurkansBool`))
        (`self.Heal` _asplayer_character_base)))))

(event `Heal`
  (params (NewParam :type "PlayerCharacterBase Object Reference"))
  (`SceneComponent.SetHiddenInGame` (`self.Niagara`) false false)
  (bind _asbp_wizard_game_state (cast `/Game/BP_WizardGameState` (`GameplayStatics.GetGameState`)))
  (`WizardGameState.RestoreHealth` _asbp_wizard_game_state (`self.Restore Amount`))
  (set `self.FurkansBool` true))

(fn `UserConstructionScript`)