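; Boss room manager that plays an intro cutscene for what appears to be the Royal Shroom boss.
; PlayCutscene waits briefly, disables input on the player character and plays the referenced Level Sequence.
; A delay matching the sequence's duration, rather than a finished event, times the restoring of input and the display of the WBP_RoyalShroomIntro widget.
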(event `self.PlayCutscene`
  (bind _sequenceplayer (`LevelSequenceActor.SequencePlayer` (`self.LevelSequence`)))
  (`KismetSystemLibrary.Delay` 3.0)
  (`self.DisableInput` (`GameplayStatics.GetPlayerCharacter` 0) null)
  (`MovieSceneSequencePlayer.Play` _sequenceplayer)
  (`KismetSystemLibrary.Delay` (`TimeManagementBlueprintLibrary.Conv_QualifiedFrameTimeToSeconds` (`MovieSceneSequencePlayer.GetDuration` _sequenceplayer)))
  (`self.EnableInput` (`GameplayStatics.GetPlayerCharacter` 0) null)
  (bind _returnvalue (`|CreateWidget` "/Game/UI/WBP_RoyalShroomIntro.WBP_RoyalShroomIntro_C"))
  (`UserWidget.AddToViewport` _returnvalue 0))

(fn `UserConstructionScript`)