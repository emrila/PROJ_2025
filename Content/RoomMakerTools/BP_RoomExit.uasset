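; Room exit actor where players vote to move on to its linked room, previewing that room's type and modifiers with icon meshes.
; Linking sets the icons and disables trigger collision; enabling resets vote state and reveals them.
; Local player overlaps report to the player controller, while RepNotifies update vote-count text and hide disabled exits.
; Exiting disables player input, advances the game instance's RoomLoader and loads the linked room after a delay.
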(event `self.ResetExitState`
  (`SceneComponent.SetVisibility` (`self.Icon`) false false)
  (`SceneComponent.SetVisibility` (`self.StaticMesh`) false false)
  (`StaticMeshComponent.SetStaticMesh` (`self.StaticMesh`) null)
  (`StaticMeshComponent.SetStaticMesh` (`self.Icon`) null))

(event `self.ReceiveBeginPlay`
  (`KismetSystemLibrary.PrintString` "RESET")
  (`self.SetActorHiddenInGame` false)
  (`self.SetActorEnableCollision` true)
  (if (`self.ExitIsDisabled`)
    (`self.HideExit`)
    (else
      (`KismetSystemLibrary.PrintString` "No"))))

(event `MulticastResetState`)

(event `HideExit`
  (`KismetSystemLibrary.PrintString` "HIDE")
  (`self.SetActorHiddenInGame` true)
  (`self.SetActorEnableCollision` false))

(event `self.DisableExit`
  (`KismetSystemLibrary.Delay` 1.25)
  (set `self.ExitIsDisabled` true))

(event `SetNoCollsion`
  (bind _icon (`self.Icon`))
  (bind _linkedroominstance_roomdata (break `RoomInstance` (`self.LinkedRoomInstance`)))
  (bind (_linkedroominstance_roomdata_2 _linkedroominstance_activemodifierclasses) (break `RoomInstance` (`self.LinkedRoomInstance`)))
  (`PrimitiveComponent.SetCollisionEnabled` (`self.Box`) "NoCollision")
  (switch `ERoomType` (`RoomData.RoomType` _linkedroominstance_roomdata)
    (:`Combat`
      (`StaticMeshComponent.SetStaticMesh` _icon "/Game/Enemy/SM_CombatIcon.SM_CombatIcon"))
    (:`Parkour`
      (`StaticMeshComponent.SetStaticMesh` _icon "/Game/Enemy/SM_ParkourIcon.SM_ParkourIcon"))
    (:`Camp`
      (`StaticMeshComponent.SetStaticMesh` _icon "/Game/Enemy/SM_CampIcon.SM_CampIcon"))
    (:`Event`
      (`StaticMeshComponent.SetStaticMesh` _icon "/Game/Enemy/SM_ChoiceIcon.SM_ChoiceIcon"))
    (:`Boss`
      (`StaticMeshComponent.SetStaticMesh` _icon "/Game/Enemy/SM_BossIcon.SM_BossIcon")))
  (for _array_element _linkedroominstance_activemodifierclasses
    (castclass `MoreEnemiesMod` _array_element
      (:`then`
        (`StaticMeshComponent.SetStaticMesh` (`self.StaticMesh`) "/Game/Enemy/SM_manyenemies2.SM_manyenemies2"))
      (:`CastFailed`
        (castclass `ParkourTimerMod` _array_element
          (:`then`
            (`StaticMeshComponent.SetStaticMesh` (`self.StaticMesh`) "/Game/Enemy/SM_2.SM_2"))
          (:`CastFailed`
            (castclass `LightsOutMod` _array_element
              (:`then`
                (`StaticMeshComponent.SetStaticMesh` (`self.StaticMesh`) "/Game/Enemy/SM_Moon.SM_Moon"))
              (:`CastFailed`
                (castclass `FallingCarrotsMod` _array_element
                  (:`then`
                    (`StaticMeshComponent.SetStaticMesh` (`self.StaticMesh`) "/Game/Enemy/SM_FallingCarrots.SM_FallingCarrots"))
                  (:`CastFailed`
                    (castclass `LowGravity` _array_element)
                    (`StaticMeshComponent.SetStaticMesh` (`self.StaticMesh`) "/Game/Enemy/SM_Arrow.SM_Arrow")))))))))))

(event `self.OnRoomLinked`
  (`self.SetNoCollsion`))

(event `self.EnableExit`
  (`self.multicast`))

(event `self.Box.OnComponentBeginOverlap`
  (params (OverlappedComponent :type "PrimitiveComponent Object Reference") (OtherActor :type "Actor Object Reference") (OtherComp :type "PrimitiveComponent Object Reference") (OtherBodyIndex :type Integer) (bFromSweep :type Boolean) (SweepResult :type "HitResult Structure (by ref)"))
  (bind _asbp_player_character_base (cast `/Game/Developer/Basir/BP_PlayerCharacterBase` OtherActor))
  (if (and (`Pawn.IsLocallyControlled` _asbp_player_character_base) (not (`self.Iscurrentlyvoting`)))
    (set `self.Iscurrentlyvoting` true)
    (bind _asbp_player_controller_base (cast `/Game/Developer/Basir/BP_PlayerControllerBase` (`GameplayStatics.GetPlayerController` 0)))
    (`/Game/Developer/Basir/BP_PlayerControllerBase.PlayerEnteredRoomExit` _asbp_player_controller_base self true)))

(event `multicast`
  (`KismetSystemLibrary.PrintText` (`|FormatText` "HasExited: {exit}, HowMany: {num}, CurrentlyVoting: {voting}" (`self.HasExited`) (`self.HowMany`) (`self.Iscurrentlyvoting`)))
  ;[0.3333 0 1 0.5] Reset to default
  (set `self.HasExited` false)
  (set `self.HowMany` 0)
  (set `self.Iscurrentlyvoting` false)
  (`PrimitiveComponent.SetCollisionEnabled` (`self.Box`) "QueryAndPhysics")
  (`SceneComponent.SetVisibility` (`self.Icon`) true false)
  (`SceneComponent.SetVisibility` (`self.StaticMesh`) true false))

(event `self.Box.OnComponentEndOverlap`
  (params (OverlappedComponent :type "PrimitiveComponent Object Reference") (OtherActor :type "Actor Object Reference") (OtherComp :type "PrimitiveComponent Object Reference") (OtherBodyIndex :type Integer))
  (bind _asbp_player_character_base (cast `/Game/Developer/Basir/BP_PlayerCharacterBase` OtherActor))
  (if (and (`Pawn.IsLocallyControlled` _asbp_player_character_base) (`self.Iscurrentlyvoting`))
    (set `self.Iscurrentlyvoting` false)
    (bind _asbp_player_controller_base (cast `/Game/Developer/Basir/BP_PlayerControllerBase` (`GameplayStatics.GetPlayerController` 0)))
    (`/Game/Developer/Basir/BP_PlayerControllerBase.PlayerEnteredRoomExit` _asbp_player_controller_base self false)))

(event `exit`
  (bind _linkedroominstance_roomdata (break `RoomInstance` (`self.LinkedRoomInstance`)))
  (`self.DisableAllPlayerMovement`)
  (bind _aswizard_game_instance (cast `WizardGameInstance` (`GameplayStatics.GetGameInstance`)))
  (bind _roomloader (`WizardGameInstance.RoomLoader` _aswizard_game_instance))
  (bind _currentroom_roomdata (break `RoomInstance` (`RoomLoader.CurrentRoom` _roomloader)))
  (`RoomLoader.RemoveRoomFromPool` _roomloader _currentroom_roomdata)
  (`RoomLoader.IncrementProgress` _roomloader true)
  (`RoomLoader.RegisterNextRoom` _roomloader _linkedroominstance_roomdata)
  (bind _roomloaderstate_onetwothreescalestate (break `RoomLoaderState` (`RoomLoader.RoomLoaderState` _roomloader)))
  (if (== _roomloaderstate_onetwothreescalestate 0)
    (`KismetSystemLibrary.Delay` 4.7)
    (else
      (`KismetSystemLibrary.Delay` 0.35)))
  (`RoomLoader.LoadNextRoom` _roomloader (`self.LinkedRoomInstance`)))

(event `DisableAllPlayerMovement`
  (`self.DisableInput` (`GameplayStatics.GetPlayerCharacter` 0) null))

(fn `OnRep_ExitIsDisabled`
  (`self.HideExit`))

(fn `OnRep_HowMany`
  (if (== (`self.HowMany`) 0)
    (`TextRenderComponent.K2_SetText` (`self.TextRender1`) "")
    (else
      (bind _asbp_wizard_game_state (cast `/Game/BP_WizardGameState` (`GameplayStatics.GetGameState`)))
      (`TextRenderComponent.K2_SetText` (`self.TextRender1`) (`KismetSystemLibrary.MakeLiteralText` (`KismetTextLibrary.Conv_StringToText` (`KismetStringLibrary.Concat_StrStr` (`KismetStringLibrary.Conv_IntToString` (`self.HowMany`)) "/" (`KismetStringLibrary.Conv_IntToString` (`KismetMathLibrary.Clamp` (`WizardGameState.CurrentPlayerCount` _asbp_wizard_game_state) 0 2)))))))))

(fn `OnRep_IsActorReplicated`
  (`self.MulticastResetState`))

(fn `UserConstructionScript`)