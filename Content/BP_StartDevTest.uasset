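; Trigger actor that launches a dev test room when a player character overlaps it.
; On the server, it builds a random room from StaticDevMapPool with the LightsOut modifier, flags the RoomLoader as a dev test, registers and loads it after a short delay, then destroys itself.
; Waiting-for-players logic is disconnected, though end overlap still clears that popup and start-dungeon state for the local player.
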(event `self.ReceiveActorBeginOverlap`
  (params (OtherActor :type "Actor Object Reference"))
  (`/Engine/EditorBlueprintResources/ActorMacros.Switch Has Authority`
    (:`Authority`
      (cast `PlayerCharacterBase` OtherActor)
      (bind _aswizard_game_instance (cast `WizardGameInstance` (`GameplayStatics.GetGameInstance`)))
      (set `self.RoomInstance` (`RoomInstanceLibrary.MakeRoomInstance` (`KismetArrayLibrary.Array_Random` (`WizardGameInstance.StaticDevMapPool` _aswizard_game_instance)) (`|MakeArray` "/Script/PROJ_2025.LightsOutMod" :!type "RoomModifierBase Class Reference")))
      (bind _aswizard_game_instance_2 (cast `WizardGameInstance` (`GameplayStatics.GetGameInstance`)))
      (set `RoomLoader.IsDevTest` true (`WizardGameInstance.RoomLoader` _aswizard_game_instance_2))
      (`self.Start`))))

(event `self.ReceiveActorEndOverlap`
  (params (OtherActor :type "Actor Object Reference"))
  (bind _asplayer_character_base (cast `PlayerCharacterBase` OtherActor))
  (if (and (`Pawn.IsLocallyControlled` _asplayer_character_base) (`KismetSystemLibrary.IsValid` (`self.waiting for others`)))
    (bind _asbp_player_controller_base (cast `/Game/Developer/Basir/BP_PlayerControllerBase` (`GameplayStatics.GetPlayerController` 0)))
    (`/Game/Developer/Basir/BP_PlayerControllerBase.EnterStartDungeon` _asbp_player_controller_base false)
    (`Widget.RemoveFromParent` (`self.waiting for others`))))

(event `self.ReceiveTick`
  (params (DeltaSeconds :type "Float (single-precision)")))

(event `AddPopup`
  (bind _returnvalue (`|CreateWidget` "/Game/UI/WBP_WaitingForOtherPlayers.WBP_WaitingForOtherPlayers_C"))
  (bind _output_get (set `self.waiting for others` _returnvalue))
  (`UserWidget.AddToViewport` _output_get 0))

(event `Start`
  (bind _roominstance_roomdata (break `RoomInstance` (`self.RoomInstance`)))
  (bind _aswizard_game_instance (cast `WizardGameInstance` (`GameplayStatics.GetGameInstance`)))
  (bind _roomloader (`WizardGameInstance.RoomLoader` _aswizard_game_instance))
  (`RoomLoader.RegisterNextRoom` _roomloader _roominstance_roomdata)
  (`KismetSystemLibrary.Delay` 0.35)
  (`RoomLoader.LoadNextRoom` _roomloader (`self.RoomInstance`))
  (`self.K2_DestroyActor`))

(fn `UserConstructionScript`)