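; Dropped loot item that launches on a random arc, scales up, spins and hovers, and can be picked up by players.
; After the drop, a multicast fills a description widget from game instance item data by row name.
; Overlaps and a sphere trace reveal the widget to local players; Tick turns it toward the camera and flags full inventories.
; Server-side collision adds the item to an inventory with free slots, then destroys the actor.
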(event `self.Initialize`
  (params (DropForceMultiplier :type "Float (single-precision)"))
  (bind _returnvalue (`self.K2_GetActorLocation`))
  (bind _returnvalue_2 (`self.K2_GetActorRotation`))
  (`KismetSystemLibrary.K2_SetTimer` null "Rotate" 7.501 true)
  (`self.Rotate`)
  (`PrimitiveComponent.AddImpulse` (`self.CollisionBox`) (* (* (`KismetMathLibrary.Normal` (+ (* (`self.GetActorForwardVector`) (`KismetMathLibrary.RandomFloatInRange` 1.5 1.8)) (* (`KismetMathLibrary.GetRightVector` _returnvalue_2) (`KismetMathLibrary.RandomFloatInRange` -1.5 1.5)) (* (`KismetMathLibrary.GetUpVector` _returnvalue_2) (`KismetMathLibrary.RandomFloatInRange` 1.7 2.0)))) 80000.0) DropForceMultiplier) "None" false)
  (bind (_direction _scalefloat) (`Timeline|Timeline` :!via `PlayFromStart`)
    (:`Update`
      (`SceneComponent.SetWorldScale3D` (`self.ItemMesh`) (`KismetMathLibrary.Conv_DoubleToVector` _scalefloat)))
    (:`Finished`
      (`KismetSystemLibrary.K2_SetTimer` null "Hover" 1.001 true)
      (`KismetSystemLibrary.Delay` 0.5)
      (`self.MulticastWidgetInfo` (`self.ItemRowName`))
      (set `self.CanPickUp` true)
      (bind _outhits (`KismetSystemLibrary.SphereTraceMultiForObjects` _returnvalue _returnvalue 650.0 (`|MakeArray` "ObjectTypeQuery8" :!type "EObjectTypeQuery Enum")))
      (for _array_element _outhits
        (bind _asplayer_character_base (cast `PlayerCharacterBase` (`.HitActor` (`GameplayStatics.BreakHitResult` _array_element))))
        (if (`Pawn.IsLocallyControlled` _asplayer_character_base)
          (`SceneComponent.SetVisibility` (`self.DescriptionWidget`) true false))))))

(event `self.ReceiveBeginPlay`
  (bind _asbp_player_character_base (cast `/Game/Developer/Basir/BP_PlayerCharacterBase` (`GameplayStatics.GetPlayerCharacter` 0)))
  (set `self.MyInventory` (`PlayerCharacterBase.Inventory` _asbp_player_character_base)))

(event `Rotate`
  (bind (_direction _newtrack_0) (`Timeline|Timeline_1` :!via `PlayFromStart`)
    (:`Update`
      (`SceneComponent.K2_SetRelativeRotation` (`self.ItemMesh`) (`KismetMathLibrary.MakeRotator` 0.0 0.0 _newtrack_0) false false))))

(event `self.ShowWidgetHere.OnComponentBeginOverlap`
  (params (OverlappedComponent :type "PrimitiveComponent Object Reference") (OtherActor :type "Actor Object Reference") (OtherComp :type "PrimitiveComponent Object Reference") (OtherBodyIndex :type Integer) (bFromSweep :type Boolean) (SweepResult :type "HitResult Structure (by ref)"))
  (bind _asbp_player_character_base (cast `/Game/Developer/Basir/BP_PlayerCharacterBase` OtherActor))
  (if (`Pawn.IsLocallyControlled` _asbp_player_character_base)
    (`SceneComponent.SetVisibility` (`self.DescriptionWidget`) true false)))

(event `Hover`
  (bind (_direction _newtrack_0) (`Timeline|Timeline_0` :!via `PlayFromStart`)
    (:`Update`
      (`SceneComponent.K2_SetRelativeLocation` (`self.ItemMesh`) (`KismetMathLibrary.MakeVector` 0.0 0.0 _newtrack_0) false false))))

(event `self.ShowWidgetHere.OnComponentEndOverlap`
  (params (OverlappedComponent :type "PrimitiveComponent Object Reference") (OtherActor :type "Actor Object Reference") (OtherComp :type "PrimitiveComponent Object Reference") (OtherBodyIndex :type Integer))
  (bind _asbp_player_character_base (cast `/Game/Developer/Basir/BP_PlayerCharacterBase` OtherActor))
  (if (`Pawn.IsLocallyControlled` _asbp_player_character_base)
    (`SceneComponent.SetVisibility` (`self.DescriptionWidget`) false false)))

(event `self.ReceiveTick`
  (params (DeltaSeconds :type "Float (single-precision)"))
  (bind _descriptionwidget (`self.DescriptionWidget`))
  (bind (_returnvalue_roll _returnvalue_pitch _returnvalue_yaw) (`KismetMathLibrary.BreakRotator` (`KismetMathLibrary.FindLookAtRotation` (`SceneComponent.K2_GetComponentLocation` _descriptionwidget) (`SceneComponent.K2_GetComponentLocation` (`PlayerCameraManager.TransformComponent` (`GameplayStatics.GetPlayerCameraManager` 0))))))
  (if (`self.CheckForInv`)
    (if (< (`KismetArrayLibrary.Array_Length` (`Inventory.Items` (`self.MyInventory`))) 2)
      (set `Widget.Visibility` "Hidden" (`/Game/UI/WorldSpace/WBP_ItemDescription.InventoryFullText` (`self.ItemWidget`)))
      (else
        (set `Widget.Visibility` "Visible" (`/Game/UI/WorldSpace/WBP_ItemDescription.InventoryFullText` (`self.ItemWidget`))))))
  (if (`KismetSystemLibrary.IsValid` (`GameplayStatics.GetPlayerPawn` 0))
    (`SceneComponent.K2_SetWorldRotation` _descriptionwidget (`KismetMathLibrary.MakeRotator` _returnvalue_roll 0.0 _returnvalue_yaw) false false)))

(event `self.CollisionBox.OnComponentBeginOverlap`
  (params (OverlappedComponent :type "PrimitiveComponent Object Reference") (OtherActor :type "Actor Object Reference") (OtherComp :type "PrimitiveComponent Object Reference") (OtherBodyIndex :type Integer) (bFromSweep :type Boolean) (SweepResult :type "HitResult Structure (by ref)"))
  (`/Engine/EditorBlueprintResources/ActorMacros.Switch Has Authority`
    (:`Authority`
      (if (`self.CanPickUp`)
        (bind _asbp_player_character_base (cast `/Game/Developer/Basir/BP_PlayerCharacterBase` OtherActor))
        (bind _inventory (`PlayerCharacterBase.Inventory` _asbp_player_character_base))
        (bind _usedslots (`Inventory.UsedSlots` _inventory))
        (if (< _usedslots 2)
          (set `Inventory.UsedSlots` (+ _usedslots 1) _inventory)
          (`Inventory.AddItem` _inventory (`self.ItemRowName`))
          (`self.K2_DestroyActor`))))))

(event `MulticastWidgetInfo`
  (params (ItemRow :type Name))
  (bind _returnvalue (`WizardGameInstance.GetItem` (`WorldGetters.GetWizardGameInstance`) ItemRow))
  (bind _aswbp_item_description (cast `/Game/UI/WorldSpace/WBP_ItemDescription` (`WidgetComponent.GetWidget` (`self.DescriptionWidget`))))
  (`Widget.SetVisibility` (`/Game/UI/WorldSpace/WBP_ItemDescription.Canvas` _aswbp_item_description) "Visible")
  (set `self.ItemWidget` _aswbp_item_description)
  (set `self.CheckForInv` true)
  (set `TextBlock.Text` (`.ItemName` (break `ItemDataRow` _returnvalue)) (`/Game/UI/WorldSpace/WBP_ItemDescription.ItemName` _aswbp_item_description))
  (set `TextBlock.Text` (`|FormatText` (`.Description` (break `ItemDataRow` _returnvalue)) " \n") (`/Game/UI/WorldSpace/WBP_ItemDescription.Description` _aswbp_item_description))
  (set `TextBlock.Text` (`KismetTextLibrary.Conv_StringToText` (`|GetEnumeratorNameAsString` (`.LootTier` (break `ItemDataRow` _returnvalue)))) (`/Game/UI/WorldSpace/WBP_ItemDescription.Rarity` _aswbp_item_description))
  (`Image.SetBrushFromTexture` (`/Game/UI/WorldSpace/WBP_ItemDescription.Icon` _aswbp_item_description) (`.Icon` (break `ItemDataRow` _returnvalue)) false)
  (`/Game/UI/WorldSpace/WBP_ItemDescription.SetBG` _aswbp_item_description (`.LootTier` (break `ItemDataRow` _returnvalue))))

(fn `UserConstructionScript`)