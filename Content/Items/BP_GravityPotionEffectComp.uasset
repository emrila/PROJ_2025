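; Gravity potion effect component that temporarily lowers the gravity of the Character it is attached to.
; On BeginPlay it saves the owner's CharacterMovement GravityScale, sets it to a fixed reduced value and waits for Duration.
; It then restores the saved scale and destroys itself.
; If the owner is not a Character, it does nothing.
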(event `self.ReceiveBeginPlay`
  (bind _ascharacter (cast `Character` (`self.GetOwner`)))
  (bind _charactermovement (`Character.CharacterMovement` _ascharacter))
  (set `self.Default Gravity` (`CharacterMovementComponent.GravityScale` _charactermovement))
  (set `CharacterMovementComponent.GravityScale` 0.5 _charactermovement)
  (`KismetSystemLibrary.Delay` (`self.Duration`))
  (set `CharacterMovementComponent.GravityScale` (`self.Default Gravity`) _charactermovement)
  (`self.K2_DestroyComponent`))