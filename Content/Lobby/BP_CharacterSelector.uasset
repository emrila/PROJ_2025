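; Lobby actor that previews one playable character class and lets a player pick it.
; Hover shows a highlight cylinder and class info widget; selecting spawns the character through the player controller and adds its HUD.
; A fast looping authority timer scans controlled pawns to hide taken previews; another clears hover visuals once the local player has a pawn.
; BlendCamera eases the view from the selector's camera to the controlled pawn.
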(event `self.ReceiveBeginPlay`
  (bind _returnvalue (`|CreateWidget` "/Game/Lobby/WBP_Character.WBP_Character_C" null self))
  (`WidgetComponent.SetWidget` (`self.Widget`) _returnvalue)
  (bind _asbp_wizard_game_state (cast `/Game/BP_WizardGameState` (`GameplayStatics.GetGameState`)))
  (set `self.GameState` _asbp_wizard_game_state)
  (`KismetSystemLibrary.K2_SetTimer` null "HideWidget" 0.01 true true)
  (`/Engine/EditorBlueprintResources/ActorMacros.Switch Has Authority`
    (:`Authority`
      (`KismetSystemLibrary.K2_SetTimer` null "HideChild" 0.01 true true)
      (`self.SetActorEnableCollision` (`ChildActorComponent.ChildActor` (`self.CharacterPreview`)) false))))

(event `Hover`
  (params (Visibility :type Boolean))
  (bind _returnvalue (`KismetSystemLibrary.IsValid` (`self.Info`)))
  (if (not (`self.bIsTaken`))
    (`SceneComponent.SetVisibility` (`self.Cylinder1`) Visibility false)
    (if Visibility
      (if (not _returnvalue)
        (bind _asbp_player_character_base (cast `/Game/Developer/Basir/BP_PlayerCharacterBase` (`ChildActorComponent.ChildActor` (`self.CharacterPreview`))))
        (bind _returnvalue_2 (`|CreateWidget` "/Game/Lobby/WBP_CharacterInfo.WBP_CharacterInfo_C" null (`PlayerCharacterBase.ClassName` _asbp_player_character_base) (`PlayerCharacterBase.ClassDescription` _asbp_player_character_base)))
        (bind _output_get (set `self.Info` _returnvalue_2))
        (`UserWidget.AddToViewport` _output_get 0))
      (elif _returnvalue
        (`Widget.RemoveFromParent` (`self.Info`))
        (set `self.Info` null)
        (`SceneComponent.SetVisibility` (`self.Cylinder1`) false false)))))

(event `SpawnCharacter`
  (bind _returnvalue (`GameplayStatics.GetPlayerController` 0))
  (bind _info (`self.Info`))
  (if (not (`self.bIsTaken`))
    (`WidgetBlueprintLibrary.SetInputMode_GameOnly` _returnvalue)
    (bind _asbp_player_controller_base (cast `/Game/Developer/Basir/BP_PlayerControllerBase` _returnvalue))
    (`/Game/Developer/Basir/BP_PlayerControllerBase.SpawnCharacter` _asbp_player_controller_base (`self.CharacterClass`) (`SceneComponent.K2_GetComponentToWorld` (`self.CharacterPreview`)) self)
    (`/Game/Developer/Basir/BP_PlayerControllerBase.AddHud` _asbp_player_controller_base (`self.CharacterWidgetClass`))
    (`self.RegisterSelection`)
    (`self.ForceNetUpdate`)
    (if (`KismetSystemLibrary.IsValid` _info)
      (`Widget.RemoveFromParent` _info)
      (set `self.Info` null))))

(event `RegisterSelection`
  (`SceneComponent.SetVisibility` (`self.Cylinder1`) false false))

(event `HideChild`
  (bind _returnvalue (`KismetArrayLibrary.Array_Contains` (`self.ActiveClasses`) (`self.CharacterClass`)))
  (`KismetArrayLibrary.Array_Clear` (`self.ActiveClasses`))
  (for _array_element (`GameStateBase.PlayerArray` (`self.GameState`))
    (bind _returnvalue_2 (`PlayerState.GetPlayerController` _array_element))
    (if (`KismetSystemLibrary.IsValid` _returnvalue_2)
      (bind _returnvalue_3 (`Controller.K2_GetPawn` _returnvalue_2))
      (if (`KismetSystemLibrary.IsValid` _returnvalue_3)
        (bind _asbp_player_character_base (castclass `/Game/Developer/Basir/BP_PlayerCharacterBase` (`GameplayStatics.GetObjectClass` _returnvalue_3)))
        (`KismetArrayLibrary.Array_Add` (`self.ActiveClasses`) _asbp_player_character_base))))
  (`SceneComponent.SetVisibility` (`self.CharacterPreview`) (not _returnvalue) false)
  (set `self.bIsTaken` _returnvalue)
  (`self.ForceNetUpdate`))

(event `HideWidget`
  (bind _info (`self.Info`))
  (if (`KismetSystemLibrary.IsValid` (`Controller.K2_GetPawn` (`GameplayStatics.GetPlayerController` 0)))
    (`SceneComponent.SetVisibility` (`self.Cylinder1`) false false)
    (if (`KismetSystemLibrary.IsValid` _info)
      (`Widget.RemoveFromParent` _info))))

(fn `BlendCamera`
  (params (Controller :type "PlayerController Object Reference"))
  (`PlayerController.SetViewTargetWithBlend` Controller (`self.Camera`) 0.0 "VTBlend_Linear" 0.0 false)
  (`PlayerController.SetViewTargetWithBlend` Controller (`Controller.K2_GetPawn` Controller) 1.0 "VTBlend_EaseIn" 1.0 false)
  (return))

(fn `UserConstructionScript`
  (`/Engine/EditorBlueprintResources/ActorMacros.Switch Has Authority`
    (:`Authority`
      (`ChildActorComponent.SetChildActorClass` (`self.CharacterPreview`) (`self.CharacterClass`)))))