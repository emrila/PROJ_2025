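; A multiplayer start-dungeon trigger that begins the run once all players are standing in it.
; On overlap, the local player reports entering or leaving through the player controller, with a waiting-for-others widget shown while inside.
; Tick compares the game state's count to the player total, then registers and loads a random normal room, picked on authority at BeginPlay, and destroys the actor.
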(event `self.ReceiveBeginPlay`
  (bind _aswizard_game_state (cast `WizardGameState` (`GameplayStatics.GetGameState`)))
  (set `self.As Wizard Game State` _aswizard_game_state)
  (`/Engine/EditorBlueprintResources/ActorMacros.Switch Has Authority`
    (:`Authority`
      (bind _aswizard_game_instance (cast `WizardGameInstance` (`GameplayStatics.GetGameInstance`)))
      (set `self.RoomInstance` (`RoomInstanceLibrary.MakeRoomInstance` (`KismetArrayLibrary.Array_Random` (`WizardGameInstance.NormalMapPool` _aswizard_game_instance)))))))

(event `self.ReceiveActorBeginOverlap`
  (params (OtherActor :type "Actor Object Reference"))
  (bind _asplayer_character_base (cast `PlayerCharacterBase` OtherActor))
  (if (`Pawn.IsLocallyControlled` _asplayer_character_base)
    (bind _asbp_player_controller_base (cast `/Game/Developer/Basir/BP_PlayerControllerBase` (`GameplayStatics.GetPlayerController` 0)))
    (`/Game/Developer/Basir/BP_PlayerControllerBase.EnterStartDungeon` _asbp_player_controller_base true)
    (`self.AddPopup`)))

(event `self.ReceiveActorEndOverlap`
  (params (OtherActor :type "Actor Object Reference"))
  (bind _asplayer_character_base (cast `PlayerCharacterBase` OtherActor))
  (if (and (`Pawn.IsLocallyControlled` _asplayer_character_base) (`KismetSystemLibrary.IsValid` (`self.waiting for others`)))
    (bind _asbp_player_controller_base (cast `/Game/Developer/Basir/BP_PlayerControllerBase` (`GameplayStatics.GetPlayerController` 0)))
    (`/Game/Developer/Basir/BP_PlayerControllerBase.EnterStartDungeon` _asbp_player_controller_base false)
    (`Widget.RemoveFromParent` (`self.waiting for others`))))

(event `self.ReceiveTick`
  (params (DeltaSeconds :type "Float (single-precision)"))
  (if (and (not (`self.HasStarted`)) (>= (`WizardGameState.PlayersInStartDungeon` (`self.As Wizard Game State`)) (`WizardGameState.CurrentPlayerCount` (`self.As Wizard Game State`))))
    (set `self.HasStarted` true)
    (`self.Start`)))

(event `AddPopup`
  (bind _returnvalue (`|CreateWidget` "/Game/UI/WBP_WaitingForOtherPlayers.WBP_WaitingForOtherPlayers_C"))
  (bind _output_get (set `self.waiting for others` _returnvalue))
  (`UserWidget.AddToViewport` _output_get 0))

(event `Start`
  (bind _roominstance_roomdata (break `RoomInstance` (`self.RoomInstance`)))
  (bind _aswizard_game_instance (cast `WizardGameInstance` (`GameplayStatics.GetGameInstance`)))
  (bind _roomloader (`WizardGameInstance.RoomLoader` _aswizard_game_instance))
  (`RoomLoader.RegisterNextRoom` _roomloader _roominstance_roomdata)
  (`KismetSystemLibrary.Delay` 0.35)
  (`RoomLoader.LoadNextRoom` _roomloader (`self.RoomInstance`))
  (`self.K2_DestroyActor`))

(fn `UserConstructionScript`)