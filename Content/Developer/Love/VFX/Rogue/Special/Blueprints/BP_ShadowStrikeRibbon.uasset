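; BP_ShadowStrikeRibbon is a Niagara ribbon VFX actor for the Rogue special, sweeping itself from a start to an end location over a given duration.
; SpawnRibbon routes through a server RPC or directly to a multicast, which activates the trail and starts a Tick-driven lerp, deactivating shortly after arrival.
; A delayed dust burst spawns below the start point, oriented by the owner's forward vector.
; Test input and unused dust logic remain.
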(event `self.ReceiveBeginPlay`
  ; For testing
)

(event `self.BP_SpawnRibbon`
  (params (StartLocation :type "Vector Structure") (EndLocation :type "Vector Structure") (Duration :type "Float (single-precision)"))
  (if (`self.HasAuthority`)
    (`self.Multicast_SpawnRibbon` StartLocation EndLocation Duration)
    (else
      (`self.Server_SpawnRibbon` StartLocation EndLocation Duration))))

(event `Multicast_SpawnRibbon`
  (params (StartLocation :type "Vector Structure") (EndLocation :type "Vector Structure") (Duration :type "Float (double-precision)"))
  ; Set rotation
  (`self.SetDustRotation`)
  (set `self.Start Location` StartLocation)
  (set `self.End Location` EndLocation)
  (set `self.Duration` Duration)
  (set `self.TimeElapsed` 0.0)
  (set `self.bIsLerping` true)
  (`ActorComponent.Activate` (`self.NS_RogueSpecial`) true)
  (`KismetSystemLibrary.Delay` 0.1)
  (`self.SpawnDustParticles`))

(event `Key|One`
  (params (Key :type "Key Structure"))
  ; Simulated values for testing purposes
  (:`Pressed`
    (set `self.Start Location` (`self.K2_GetActorLocation`))
    (set `self.End Location` (+ (`self.K2_GetActorLocation`) (`KismetMathLibrary.MakeVector` 1000.0 1000.0 1000.0)))
    (set `self.Duration` 0.2)))

(event `self.ReceiveTick`
  (params (DeltaSeconds :type "Float (single-precision)"))
  (if (`self.bIsLerping`)
    (bind _output_get (set `self.TimeElapsed` (+ DeltaSeconds (`self.TimeElapsed`))))
    (bind _output_get_2 (set `self.Alpha` (`KismetMathLibrary.FClamp` (/ _output_get (`self.Duration`)))))
    (`self.K2_SetActorLocation` (`KismetMathLibrary.VLerp` (`self.Start Location`) (`self.End Location`) _output_get_2) true)
    (if (>= (`self.Alpha`) 1.0)
      (set `self.bIsLerping` false)
      (`KismetSystemLibrary.Delay` 0.05)
      (`ActorComponent.Deactivate` (`self.NS_RogueSpecial`)))))

(event `SetDustRotation`
  (bind _returnvalue (`self.GetOwner`))
  (`/Engine/EditorBlueprintResources/StandardMacros.IsValid` _returnvalue
    (:`Is Valid`
      (set `self.DustRotation` (`KismetMathLibrary.Conv_VectorToRotator` (`self.GetActorForwardVector` _returnvalue))))))

(event `Server_SpawnRibbon`
  (params (StartLocation :type "Vector Structure") (EndLocation :type "Vector Structure") (Duration :type "Float (double-precision)"))
  (`self.Multicast_SpawnRibbon` StartLocation EndLocation Duration))

(event `SpawnDustParticles`
  (`NiagaraFunctionLibrary.SpawnSystemAtLocation` (`self.NS_RogueSpecialDust`) (- (`self.Start Location`) (0.0 0.0 50.0)) (`self.DustRotation`) (2.0 2.0 2.0)))

(fn `UserConstructionScript`)