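; BP_MageSpecialSpawner is a spawner actor for the Mage special ability's Chrono Rift Niagara effect.
; SpawnChronoRift spawns the system inactive at the actor's location, then sets its radius, normalized by a base unit size, and its duration as user variables.
; It activates the effect only after those are set, then destroys itself, leaving the unattached system to play independently.
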(fn `SpawnChronoRift`
  (params (ChronoRadius :type "Float (double-precision)") (ChronoDuration :type "Float (double-precision)"))
  (locals (NiagaraInstance :type "NiagaraComponent Object Reference"))
  (bind _returnvalue (`NiagaraFunctionLibrary.SpawnSystemAtLocation` (`self.NS_MageSpecial`) (`self.K2_GetActorLocation`) (struct) (1.0 1.0 1.0) true false))
  (bind _output_get (set `local.NiagaraInstance` _returnvalue))
  (`NiagaraComponent.SetVariableFloat` _output_get (`self.ChronoRadius`) (/ ChronoRadius (`self.BaseRadiusUnits`)))
  (`NiagaraComponent.SetVariableFloat` (`local.NiagaraInstance`) (`self.ChronoDuration`) ChronoDuration)
  (`ActorComponent.Activate` (`local.NiagaraInstance`) false)
  (`self.K2_DestroyActor`))

(fn `UserConstructionScript`)