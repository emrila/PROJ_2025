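; Developer actor that repeatedly spawns a projectile Blueprint at its own location, apparently for previewing projectile VFX.
; On BeginPlay it spawns one projectile immediately, then a looping timer repeats the spawn at a configurable interval.
; Every spawn uses a fixed rotation, independent of the spawner's own orientation.
; A separate ApplyText event copies the Title variable into a text render component as a label.
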(event `self.ReceiveBeginPlay`
  (`self.SpawnProjectileVFX`)
  (`KismetSystemLibrary.K2_SetTimerDelegate` (delegate `SpawnProjectileVFX`) (`self.ProjectileSpawnInterval`) true))

(event `SpawnProjectileVFX`
  (`|SpawnActorFromClass` (`self.ProjectileBP`) (`KismetMathLibrary.MakeTransform` (`self.K2_GetActorLocation`) (struct :`Yaw` 90.0)) "Undefined" "MultiplyWithRoot" null null))

(event `ApplyText`
  (`TextRenderComponent.K2_SetText` (`self.TextRender`) (`self.Title`)))

(fn `UserConstructionScript`)