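; Spike trap that rises shortly after anything overlaps its trigger box and hurts characters that touch its damage box.
; A timer fires the raise Timeline, which offsets the spikes vertically from their starting location, then a second Timeline lowers them after a pause, with DoOnce blocking retriggers until finished.
; The damage box reduces mage health through BP_WizardGameState and launches the mage backward and upward, while mushrooms take damage directly.
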(event `self.ReceiveBeginPlay`
  (set `self.SpikeBaseLocation` (`SceneComponent.K2_GetComponentLocation` (`self.Spikes`))))

(event `self.Box.OnComponentBeginOverlap`
  (params (OverlappedComponent :type "PrimitiveComponent Object Reference") (OtherActor :type "Actor Object Reference") (OtherComp :type "PrimitiveComponent Object Reference") (OtherBodyIndex :type Integer) (bFromSweep :type Boolean) (SweepResult :type "HitResult Structure (by ref)"))
  (`KismetSystemLibrary.K2_SetTimerDelegate` (delegate `RaiseSpikes`) 0.5))

(event `RaiseSpikes`
  (`/Engine/EditorBlueprintResources/StandardMacros.DoOnce` false :!label _label
    (:`Completed`
      (bind (_direction _newtrack_0) (`Timeline|Timeline` :!via `PlayFromStart`)
        (:`Update`
          (`SceneComponent.K2_SetWorldLocation` (`self.Spikes`) (+ (`self.SpikeBaseLocation`) (`KismetMathLibrary.MakeVector` 0.0 0.0 _newtrack_0)) false false))
        (:`Finished`
          (`KismetSystemLibrary.Delay` 4.0)
          (bind (_direction_2 _newtrack_0_2) (`Timeline|Timeline_0` :!via `ReverseFromEnd`)
            (:`Update`
              (`SceneComponent.K2_SetWorldLocation` (`self.Spikes`) (+ (`self.SpikeBaseLocation`) (`KismetMathLibrary.MakeVector` 0.0 0.0 _newtrack_0_2)) false false))
            (:`Finished`
              (goto _label :!via `Reset`))))))))

(event `self.Box1.OnComponentBeginOverlap`
  (params (OverlappedComponent :type "PrimitiveComponent Object Reference") (OtherActor :type "Actor Object Reference") (OtherComp :type "PrimitiveComponent Object Reference") (OtherBodyIndex :type Integer) (bFromSweep :type Boolean) (SweepResult :type "HitResult Structure (by ref)"))
  (bind _asbp_mage_character (cast `/Game/Basir/BP_MageCharacter` OtherActor)
    (:`then`
      (bind _asbp_wizard_game_state (cast `/Game/BP_WizardGameState` (`GameplayStatics.GetGameState`)))
      (`WizardGameState.DamageHealth` _asbp_wizard_game_state 20.0)
      (bind (_returnvalue_x _returnvalue_y) (`KismetMathLibrary.BreakVector` (* (`self.GetActorForwardVector` _asbp_mage_character) -1000.0)))
      (`Character.LaunchCharacter` _asbp_mage_character (`KismetMathLibrary.MakeVector` _returnvalue_x _returnvalue_y 500.0) false false))
    (:`CastFailed`
      (bind _asbp_mushroom (cast `/Game/Enemy/BP_Mushroom` OtherActor))
      (`MushroomCharacter.TakeDamage` _asbp_mushroom 20.0 (make `DamageEvent`) null null))))

(fn `UserConstructionScript`)