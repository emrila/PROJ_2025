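; BP_CharacterSelector is a placed actor offering one playable character class, shown as a child actor preview set at construction alongside a WBP_Character widget.
; A fast looping timer polls pawn classes in the GameState's PlayerArray, hiding the preview and marking it taken when its class is in use.
; While free, hovering toggles a cylinder highlight, and selection adds the HUD and spawns the character at the preview's transform through the player controller.
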(event `self.ReceiveBeginPlay`
  (bind _returnvalue (`|CreateWidget` "/Game/Developer/Robin/WBP_Character.WBP_Character_C" null self))
  (`WidgetComponent.SetWidget` (`self.Widget`) _returnvalue)
  (`KismetSystemLibrary.K2_SetTimer` null "HideChild" 0.01 true true)
  (bind _asbp_wizard_game_state (cast `/Game/BP_WizardGameState` (`GameplayStatics.GetGameState`)))
  (set `self.GameState` _asbp_wizard_game_state))

(event `HideChild`
  (bind _returnvalue (`KismetArrayLibrary.Array_Contains` (`self.ActiveClasses`) (`self.CharacterClass`)))
  (`KismetArrayLibrary.Array_Clear` (`self.ActiveClasses`))
  (for _array_element (`GameStateBase.PlayerArray` (`self.GameState`))
    (bind _returnvalue_2 (`PlayerState.GetPlayerController` _array_element))
    (if (`KismetSystemLibrary.IsValid` _returnvalue_2)
      (bind _returnvalue_3 (`Controller.K2_GetPawn` _returnvalue_2))
      (if (`KismetSystemLibrary.IsValid` _returnvalue_3)
        (bind _asbp_player_character_base (castclass `/Game/Developer/Basir/BP_PlayerCharacterBase` (`GameplayStatics.GetObjectClass` _returnvalue_3)))
        (`KismetArrayLibrary.Array_Add` (`self.ActiveClasses`) _asbp_player_character_base))))
  (`SceneComponent.SetVisibility` (`self.CharacterPreview`) (not _returnvalue) false)
  (set `self.bIsTaken` _returnvalue))

(event `Hover`
  (params (Visibility :type Boolean))
  (if (not (`self.bIsTaken`))
    (`SceneComponent.SetVisibility` (`self.Cylinder1`) Visibility false)))

(event `SpawnCharacter`
  (bind _returnvalue (`GameplayStatics.GetPlayerController` 0))
  (if (not (`self.bIsTaken`))
    (`self.HideChild`)
    (`WidgetBlueprintLibrary.SetInputMode_GameOnly` _returnvalue)
    (bind _asbp_player_controller_base (cast `/Game/Developer/Basir/BP_PlayerControllerBase` _returnvalue))
    (`/Game/Developer/Basir/BP_PlayerControllerBase.AddHud` _asbp_player_controller_base (`self.CharacterWidgetClass`))
    (`/Game/Developer/Basir/BP_PlayerControllerBase.SpawnCharacter` _asbp_player_controller_base (`self.CharacterClass`) (`SceneComponent.K2_GetComponentToWorld` (`self.CharacterPreview`)))
    (`self.RegisterSelection`)))

(event `RegisterSelection`
  (set `self.bIsTaken` true))

(fn `UserConstructionScript`
  (`ChildActorComponent.SetChildActorClass` (`self.CharacterPreview`) (`self.CharacterClass`)))