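; Base player character for a wizard game, providing an overhead-style name tag, widget interaction, inventory toggling and hit feedback.
; On possession it fills the tag from the LAN or player-state name; separate events hide it or turn it toward the camera.
; Construction creates dynamic mesh materials, whose damage parameter HitFeedback briefly toggles to flash the character.
; Interact input simulates left clicks through WidgetInteraction, while I or Tab toggles the inventory.
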(event `AdjustWidget`
  (bind _playernametagwidgetcomponent (`self.PlayerNameTagWidgetComponent`))
  (`SceneComponent.K2_SetWorldRotation` _playernametagwidgetcomponent (`KismetMathLibrary.FindLookAtRotation` (`SceneComponent.K2_GetComponentLocation` _playernametagwidgetcomponent) (`SceneComponent.K2_GetComponentLocation` (`PlayerCameraManager.TransformComponent` (`GameplayStatics.GetPlayerCameraManager` 0)))) false false))

(event `self.ReceiveBeginPlay`
  (cast `/Game/BP_WizardGameState` (`GameplayStatics.GetGameState`))
  (`self.SetName` (`self.Name`)))

(event `self.ReceivePossessed`
  (params (NewController :type "Controller Object Reference"))
  (bind _returnvalue (`KismetTextLibrary.Conv_StringToText` (`AdvancedSessionsLibrary.GetPlayerName` (`self.PlayerController`))))
  (bind _returnvalue_2 (`KismetTextLibrary.Conv_StringToText` (`WizardPlayerState.LanPlayerName` (`self.ThePlayerState`))))
  (bind _asplayer_controller (cast `PlayerController` NewController))
  (bind _output_get (set `self.PlayerController` _asplayer_controller))
  (bind _aswizard_player_state (cast `WizardPlayerState` (`Controller.PlayerState` _output_get)))
  (set `self.ThePlayerState` _aswizard_player_state)
  (bind _asbp_wizard_game_instance (cast `/Game/BP_WizardGameInstance` (`GameplayStatics.GetGameInstance`)))
  (if (`WizardGameInstance.bIsLanGame` _asbp_wizard_game_instance)
    (`self.SetName` _returnvalue_2)
    (set `self.Name` _returnvalue_2)
    (else
      (`KismetSystemLibrary.PrintText` _returnvalue)
      (`self.SetName` _returnvalue)
      (set `self.Name` _returnvalue))))

(event `SetName`
  (params (Name :type Text))
  (bind _aswbp_player_tag (cast `/Game/UI/Player/WBP_PlayerTag` (`WidgetComponent.GetWidget` (`self.PlayerNameTagWidgetComponent`))))
  (set `TextBlock.Text` Name (`/Game/UI/Player/WBP_PlayerTag.TextBlock_NameTag` _aswbp_player_tag)))

(event `HideName`
  (`SceneComponent.SetVisibility` (`self.PlayerNameTagWidgetComponent`) false false))

(event `EnhancedInput|/Game/Input/Actions/IA_Interact`
  (params (ActionValue :type Boolean) (ElapsedSeconds :type "Float (double-precision)") (TriggeredSeconds :type "Float (double-precision)") (InputAction :type "InputAction Object Reference" :default "/Game/Input/Actions/IA_Interact.IA_Interact"))
  (bind _widgetinteraction (`self.WidgetInteraction`))
  (:`Started`
    (`WidgetInteractionComponent.PressPointerKey` _widgetinteraction "LeftMouseButton"))
  (:`Canceled`
    (`WidgetInteractionComponent.ReleasePointerKey` _widgetinteraction "LeftMouseButton" :!label _label))
  (:`Completed`
    (goto _label)))

(event `self.HitFeedback`
  (for _array_element (`self.DynamicMaterials`)
    (`MaterialInstanceDynamic.SetScalarParameterValue` _array_element "DamageToggle" 1.0))
  (`KismetSystemLibrary.Delay` 0.1)
  (for _array_element_2 (`self.DynamicMaterials`)
    (`MaterialInstanceDynamic.SetScalarParameterValue` _array_element_2 "DamageToggle" 0.0)))

(event `Key|I`
  (params (Key :type "Key Structure"))
  (:`Pressed`
    (`Inventory.ToggleInventory` (`self.Inventory`))))

(event `Key|Tab`
  (params (Key :type "Key Structure"))
  (:`Pressed`
    (`Inventory.ToggleInventory` (`self.Inventory`))))

(fn `UserConstructionScript`
  (bind _returnvalue (`self.GetComponentByClass` "/Script/Engine.SkeletalMeshComponent"))
  (for (_array_element _array_index) (`MeshComponent.GetMaterials` _returnvalue)
    (bind _returnvalue_2 (`PrimitiveComponent.CreateDynamicMaterialInstance` _returnvalue _array_index _array_element "None"))
    (`PrimitiveComponent.SetMaterial` _returnvalue _array_index _returnvalue_2)
    (`KismetArrayLibrary.Array_Add` (`self.DynamicMaterials`) _returnvalue_2)))