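; Chrono rift actor that spawns the mage special Niagara effect at its own location when SpawnEffect is called.
; SpawnEffect stores the duration, base radius and current radius, then creates the system inactive.
; It passes the current-to-base radius ratio and the duration to the ChronoRadius and ChronoDuration parameters before activating it, so the effect starts with those values.
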(event `self.BP_SpawnEffect`
  (params (NewChronoDuration :type "Float (single-precision)") (BaseRadius :type "Float (single-precision)") (CurrentRadius :type "Float (single-precision)"))
  (set `self.NewChronoDuration` NewChronoDuration)
  (set `self.Current Radius` CurrentRadius)
  (set `self.Base Radius` BaseRadius)
  (bind _returnvalue (`NiagaraFunctionLibrary.SpawnSystemAtLocation` (`self.NS_MageSpecial`) (`self.K2_GetActorLocation`) (struct) (1.0 1.0 1.0) true false))
  (bind _output_get (set `self.NiagaraInstance` _returnvalue))
  (`NiagaraComponent.SetVariableFloat` _output_get (`self.ChronoRadius`) (/ (`self.Current Radius`) (`self.Base Radius`)))
  (`NiagaraComponent.SetVariableFloat` (`self.NiagaraInstance`) (`self.ChronoDuration`) (`self.NewChronoDuration`))
  (`ActorComponent.Activate` (`self.NiagaraInstance`) false))

(fn `UserConstructionScript`)