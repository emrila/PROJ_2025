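; Player controller for a multiplayer wizard game, handling character spawning and possession, HUD setup, menu toggling and proximity-style voice chat.
; BeginPlay caches the game state and starts networked voice; VOIP registration retries until the PlayerState is valid, then applies optional attenuation and effects.
; Votes and start-dungeon entry are forwarded to BP_WizardGameState.
; Room exits track occupant counts and fire once enough players, capped at two, are inside.
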(event `self.ReceiveBeginPlay`
  (bind _aswizard_game_state (cast `WizardGameState` (`GameplayStatics.GetGameState`)))
  (set `self.Gamestate` _aswizard_game_state)
  (`self.ToggleVoice`))

(event `StartVoice`
  ; Voice
  (if (`self.IsLocalPlayerController`)
    (`KismetSystemLibrary.ExecuteConsoleCommand` "voice.MicInputGain 3" null)
    (`KismetSystemLibrary.ExecuteConsoleCommand` "ToggleSpeaking 1" null)
    (`GameplayStatics.SetBaseSoundMix` "/Game/VoiceChat/SCM_Voice.SCM_Voice")))

(event `CheckActiveCharacter`
  (if (`KismetSystemLibrary.IsValid` (`GameplayStatics.GetPlayerCharacter` 0))
    (set `self.bShowMouseCursor` false)
    (else
      (set `self.bShowMouseCursor` true))))

(event `Init VOIP`
  (bind _returnvalue (`GameplayStatics.GetPlayerState` 0))
  ; Voice
  (`/Engine/EditorBlueprintResources/StandardMacros.IsValid` _returnvalue :!label _label
    (:`Is Valid`
      (`VOIPTalker.RegisterWithPlayerState` (`self.VOIPTalker`) _returnvalue)
      (`VOIPStatics.SetMicThreshold` -1.5)
      (set `VOIPTalker.Settings` (select `/Game/VoiceChat/E_Voice` (`self.Voice`) :`NewEnumerator0` (make `VoiceSettings` null) :`NewEnumerator1` (make `VoiceSettings` null "/Game/VoiceChat/SA_Voice.SA_Voice" "/Game/VoiceChat/SEPC_Voice.SEPC_Voice")) (`self.VOIPTalker`))
      (`KismetSystemLibrary.PrintString` "Player Registered"))
    (:`Is Not Valid`
      (`KismetSystemLibrary.RetriggerableDelay` 0.2)
      (goto _label))))

(event `EnhancedInput|/Game/Input/Actions/IA_ToggleMenu`
  (params (ActionValue :type Boolean) (ElapsedSeconds :type "Float (double-precision)") (TriggeredSeconds :type "Float (double-precision)") (InputAction :type "InputAction Object Reference" :default "/Game/Input/Actions/IA_ToggleMenu.IA_ToggleMenu"))
  ;[0.5 0 1 0.5] INPUT - TOGGLE MENU
  (:`Triggered`
    (`self.bOnMenuCooldown`
      (:`then`)
      (:`else`
        (set `self.bOnMenuCooldown` true)
        (message `PlayerHUDInterface.ToggleWidget` (`self.GetHUD`) 0)
        (`KismetSystemLibrary.K2_SetTimerDelegate` (delegate `ResetMenuCooldown_Event`) 0.01)))))

(event `ResetMenuCooldown_Event`
  ;[0.5 0 1 0.5] INPUT - TOGGLE MENU
  (set `self.bOnMenuCooldown` false))

(event `AddHealthbar`
  (bind _returnvalue (`|CreateWidget` "/Game/UI/Player/WBP_PlayerHealthbar.WBP_PlayerHealthbar_C"))
  (set `self.Healthbar` _returnvalue)
  (`UserWidget.AddToViewport` _returnvalue 0))

(event `SetVoiceMode`
  (params (Voice :type "/Game/VoiceChat/E_Voice Enum" :default "NewEnumerator0"))
  ; Voice
  (set `self.Voice` Voice))

(event `SpawnCharacter`
  (params (CharacterClass :type "/Game/Developer/Basir/BP_PlayerCharacterBase Class Reference") (Transform :type "Transform Structure"))
  (bind _returnvalue (`|SpawnActorFromClass` CharacterClass Transform "Undefined" "MultiplyWithRoot" self null))
  (`self.Possess` _returnvalue))

(event `Vote`
  (params (Candidate :type "Candidate Structure"))
  (bind _asbp_wizard_game_state (cast `/Game/BP_WizardGameState` (`GameplayStatics.GetGameState`)))
  (`/Game/BP_WizardGameState.Vote` _asbp_wizard_game_state Candidate))

(event `ToggleVoice`
  ; Voice
  (`self.VOIPTalker`
    (:`then`
      (`self.SetVoiceMode` "NewEnumerator1")
      (`AdvancedVoiceLibrary.StartNetworkedVoice` 0)
      (`KismetSystemLibrary.PrintString` "Started Voice Chat"))
    (:`else`)))

(event `AddHud`
  (params (WidegetClass :type "UserWidget Class Reference"))
  (bind _returnvalue (`|CreateWidget` WidegetClass self))
  ;[0.1667 0 1] EDIT
  (`UserWidget.AddToViewport` _returnvalue 0)
  ;[0.3333 0 1 0.5] Create HUD (if not set correctly) and create widgets
  (`self.ClientSetHUD` "/Game/Developer/Emma/BP_PlayerHUD.BP_PlayerHUD_C")
  (message `PlayerHUDInterface.InitWidgets` (`self.GetHUD`)))

(event `EnterStartDungeon`
  (params (`Entered?` :type Boolean))
  (bind _asbp_wizard_game_state (cast `/Game/BP_WizardGameState` (`GameplayStatics.GetGameState`)))
  (`WizardGameState.PlayerEnteredStartDungeon` _asbp_wizard_game_state `Entered?`))

(event `CloseVoice`
  (bind _returnvalue (`GameplayStatics.GetPlayerState` 0))
  ; Voice
  (`self.VOIPTalker`
    (:`then`
      (if (!= (`self.Voice`) 0)
        (`KismetSystemLibrary.ExecuteConsoleCommand` "ToggleSpeaking 0" (`PlayerState.GetPlayerController` _returnvalue))
        (`AdvancedVoiceLibrary.MuteRemoteTalker` 0 (`AdvancedSessionsLibrary.GetUniqueNetIDFromPlayerState` _returnvalue) true)
        (`AdvancedVoiceLibrary.RemoveAllRemoteTalkers`)
        (`VoiceLibrary.ClearVoicePackage` self)))
    (:`else`)))

(event `PlayerEnteredRoomExit`
  (params (RoomExit :type "/Game/RoomMakerTools/BP_RoomExit Object Reference") (`Entered?` :type Boolean))
  (bind _howmany (`/Game/RoomMakerTools/BP_RoomExit.HowMany` RoomExit))
  (bind _textrender1 (`/Game/RoomMakerTools/BP_RoomExit.TextRender1` RoomExit))
  (if (`KismetSystemLibrary.IsValid` RoomExit)
    (if `Entered?`
      (set `/Game/RoomMakerTools/BP_RoomExit.HowMany` (+ _howmany 1) RoomExit)
      (else
        (set `/Game/RoomMakerTools/BP_RoomExit.HowMany` (- _howmany 1) RoomExit)))
    (if (== _howmany 0)
      (`TextRenderComponent.K2_SetText` _textrender1 "")
      (else
        (bind _asbp_wizard_game_state (cast `/Game/BP_WizardGameState` (`GameplayStatics.GetGameState`)))
        (bind _returnvalue (`KismetMathLibrary.Clamp` (`WizardGameState.CurrentPlayerCount` _asbp_wizard_game_state) 0 2))
        (`TextRenderComponent.K2_SetText` _textrender1 (`KismetSystemLibrary.MakeLiteralText` (`KismetTextLibrary.Conv_StringToText` (`KismetStringLibrary.Concat_StrStr` (`KismetStringLibrary.Conv_IntToString` (`/Game/RoomMakerTools/BP_RoomExit.HowMany` RoomExit)) "/" (`KismetStringLibrary.Conv_IntToString` _returnvalue)))))
        (if (and (>= _howmany _returnvalue) (not (`/Game/RoomMakerTools/BP_RoomExit.HasExited` RoomExit)))
          (set `/Game/RoomMakerTools/BP_RoomExit.HasExited` true RoomExit)
          (`/Game/RoomMakerTools/BP_RoomExit.exit` RoomExit)
          (`KismetSystemLibrary.PrintString` "uhhhh"))))))

(fn `UserConstructionScript`)