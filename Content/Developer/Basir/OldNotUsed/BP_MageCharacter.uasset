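; Networked mage player character that adds a healthbar widget, displays the profile username and takes mushroom hits.
; The local player sends a temporary random-number name to the server; its OnRep fills the name-tag widget, retrying until valid.
; Non-local characters turn their tags toward the camera each tick.
; Mushroom overlaps launch player 0 away, damage health through WizardGameState and start timed i-frames, though the i-frame check is disconnected.
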(event `self.ReceiveBeginPlay`
  (bind (_returnvalue_steamid _returnvalue_username) (break `PlayerProfile` (`PlayerLoginSystem.GetProfile` (subsystem `PlayerLoginSystem`))))
  (bind _returnvalue (`|CreateWidget` "/Game/UI/Player/WBP_PlayerHealthbar.WBP_PlayerHealthbar_C" (`GameplayStatics.GetPlayerController` 0)))
  (`UserWidget.AddToViewport` _returnvalue 0)
  (`TextRenderComponent.K2_SetText` (`self.TextRender`) (`KismetTextLibrary.Conv_StringToText` _returnvalue_username))
  (`self.SetUpLocal`))

(event `SetPlayerNameOnServer`
  (params (CustomPlayerName :type Text))
  (set `self.CustomPlayerName` CustomPlayerName))

(event `self.ReceiveActorBeginOverlap`
  (params (OtherActor :type "Actor Object Reference"))
  (bind _asbp_mushroom (cast `/Game/Enemy/Mushroom/BP_Mushroom` OtherActor))
  (bind _asplayer_character_base (cast `PlayerCharacterBase` (`GameplayStatics.GetPlayerCharacter` 0)))
  (bind (_returnvalue_x _returnvalue_y) (`KismetMathLibrary.BreakVector` (* (`KismetMathLibrary.Normal` (- (`self.K2_GetActorLocation` _asbp_mushroom) (`self.K2_GetActorLocation`))) -1000.0)))
  (`self.LaunchCharacter` _asplayer_character_base (`KismetMathLibrary.MakeVector` _returnvalue_x _returnvalue_y 100.0) false false)
  (bind _aswizard_game_state (cast `WizardGameState` (`GameplayStatics.GetGameState`)))
  (`WizardGameState.DamageHealth` _aswizard_game_state 10.0)
  (set `self.HasIframes` true)
  (`KismetSystemLibrary.K2_SetTimer` null "ResetIframes" 1.0))

(event `ResetIframes`
  (set `self.HasIframes` false))

(event `self.ReceiveTick`
  (params (DeltaSeconds :type "Float (single-precision)"))
  (`self.TickNotLocal`))

(fn `OnRep_CustomPlayerName`
  (bind _returnvalue (`WidgetComponent.GetWidget` (`self.PlayerNameTagWidget`)))
  (`/Engine/EditorBlueprintResources/StandardMacros.IsValid` _returnvalue
    (:`Is Valid`
      (bind _aswbp_player_name_tag (cast `/Game/UI/Player/WBP_PlayerNameTag` _returnvalue))
      (`/Game/UI/Player/WBP_PlayerNameTag.SetPlayerTag` _aswbp_player_name_tag (`self.CustomPlayerName`)))
    (:`Is Not Valid`
      (`KismetSystemLibrary.K2_SetTimer` null "OnRep_CustomPlayerName" 0.1))))

(fn `SetUpLocal`
  (if (`self.IsLocallyControlled`)
    (`self.SetPlayerNameOnServer` (`KismetTextLibrary.Conv_IntToText` (`KismetMathLibrary.RandomInteger` 10)))))

(fn `TickNotLocal`
  ;[0.05 0 0.15 0.5] Face (other) players camera
  (if (not (`self.IsLocallyControlled`))
    (`SceneComponent.K2_SetWorldRotation` (`self.PlayerNameTagWidget`) (`KismetMathLibrary.FindLookAtRotation` (`SceneComponent.K2_GetComponentLocation` (`self.PlayerNameTagWidget`)) (`self.K2_GetActorLocation` (`GameplayStatics.GetPlayerCameraManager` 0))) false false)))

(fn `UserConstructionScript`)