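; Rogue player character Blueprint that equips itself with a dagger, which starts out hidden.
; On BeginPlay, after the parent logic, it spawns a BP_Dagger owned by itself, stores it, attaches it to the mesh's R_HandSocket and hides it in game.
; Overlap and Tick are disabled, the construction script only calls the parent, and an unused attach to HandGrip_R is left disconnected.
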(event `self.ReceiveBeginPlay`
  (`parent.ReceiveBeginPlay`)
  (bind _returnvalue (`|SpawnActorFromClass` "/Game/Developer/Basir/Items/BP_Dagger.BP_Dagger_C" (`SkinnedMeshComponent.GetBoneTransform` (`self.Mesh`) (`SkinnedMeshComponent.GetSocketBoneName` (`self.Mesh`) "R_HandSocket") "RTS_ParentBoneSpace") "Undefined" "MultiplyWithRoot" self null))
  (bind _output_get (set `self.Dagger` _returnvalue))
  (`self.K2_AttachToComponent` _output_get (`self.Mesh`) "R_HandSocket" "KeepRelative" "KeepRelative" "KeepRelative" true)
  (`self.SetActorHiddenInGame` _output_get true))

(fn `UserConstructionScript`
  (`parent.UserConstructionScript`))