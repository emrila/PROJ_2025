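; Chrono rift actor that, judging by its asset names, serves as the orb of the Mage's special ability.
; On BeginPlay it plays the MageSpecialOrb audio event attached to its sphere component.
; An unconnected chain that never runs would spawn the NSMageSpecial Niagara system, set its radius scale and duration parameters, then activate it.
; The Blueprint graphs contain no overlap, tick or time-manipulation logic.
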(event `self.ReceiveBeginPlay`
  (`FMODBlueprintStatics.PlayEventAttached` "/Game/FMOD/Events/Players/Mage/MageSpecialOrb.MageSpecialOrb" (`self.SphereComponent`) "None" (0.0 0.0 0.0) "KeepRelativeOffset"))

(fn `UserConstructionScript`)