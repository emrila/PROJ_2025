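; Dash attack component for BP_PlayerCharacterRogue that drives the dash visual effects: a Niagara ribbon trail and a dust burst below the character.
; On BeginPlay it caches the owner's DashRibbon and binds to OnDash, which multicasts dust and a briefly activated ribbon.
; A separate server-to-multicast path toggles the ribbon, spawning dust on activation and delaying deactivation slightly.
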(event `self.ReceiveBeginPlay`
  (bind _asbp_player_character_rogue (cast `/Game/Developer/Basir/BP_PlayerCharacterRogue` (`self.GetOwner`))
    (:`then`
      (`/Engine/EditorBlueprintResources/StandardMacros.IsValid` _asbp_player_character_rogue
        (:`Is Valid`
          (bind _output_get (set `self.Player` _asbp_player_character_rogue))
          (set `self.RibbonNiagara` (`/Game/Developer/Basir/BP_PlayerCharacterRogue.DashRibbon` _output_get))
          (add `PlayerCharacterBase.OnDash` (`self.Player`) (delegate `HandleRibbon`)))))
    (:`CastFailed`
      (`KismetSystemLibrary.PrintString` "Cast in DashComp Eventgraph Failed" true true (struct :`R` 1.0 :`G` 0.978402 :`A` 1.0) 50.0))))

(event `HandleRibbon`
  (`self.Multicast_HandleRibbon`))

(event `Multicast_HandleRibbon`
  (bind _ribbonniagara (`self.RibbonNiagara`))
  (`self.SpawnDustNiagara`)
  ; Also try without resetting
  (`/Engine/EditorBlueprintResources/StandardMacros.IsValid` _ribbonniagara
    (:`Is Valid`
      (`self.Activate` _ribbonniagara true)
      (`KismetSystemLibrary.Delay` 0.3)
      (`self.Deactivate` _ribbonniagara))))

(event `SetRibbonActive`
  (params (bShouldActivate :type Boolean))
  (bind _ribbonniagara (`self.RibbonNiagara`))
  (`/Engine/EditorBlueprintResources/StandardMacros.IsValid` (`self.RibbonNiagara`)
    (:`Is Valid`
      (if bShouldActivate
        (`self.SpawnDustNiagara`)
        (`self.Activate` _ribbonniagara true)
        (else
          (`KismetSystemLibrary.Delay` 0.1)
          (`self.Deactivate` _ribbonniagara))))
    (:`Is Not Valid`
      (`KismetSystemLibrary.PrintString` "Ribbon is not valid" true true (struct :`R` 1.0 :`G` 0.78781 :`A` 1.0) 50.0))))

(event `Server_SetRibbonActive`
  (params (bShouldActivate :type Boolean))
  (`KismetSystemLibrary.PrintString` "Sever Called" true true (struct :`R` 1.0 :`G` 0.78781 :`A` 1.0) 50.0)
  (`self.Multicast_SetRibbonActive` bShouldActivate))

(event `Multicast_SetRibbonActive`
  (params (bShouldActivate :type Boolean))
  (`self.SetRibbonActive` bShouldActivate))

(event `SpawnDustNiagara`
  (`NiagaraFunctionLibrary.SpawnSystemAtLocation` "/Game/Developer/Love/VFX/Rogue/Special/NS_RogueSpecialDust.NS_RogueSpecialDust" (- (`Actor.K2_GetActorLocation` (`self.Player`)) (0.0 0.0 50.0))))