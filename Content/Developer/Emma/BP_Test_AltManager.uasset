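; Debug test actor that displays the state of its ValidationComponent's selectables through text renderers.
; On authority it waits for SelectionTag gameplay events, then stores each selectable's total selector count in ChildTexts when the counts change.
; An OnRep on ChildTexts refreshes the children text for replication.
; Tick shows a countdown with the evaluation tag while the component's selection evaluation timer is active, and hides it otherwise.
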(event `self.ReceiveBeginPlay`
  (`parent.ReceiveBeginPlay`)
  (`TextRenderComponent.K2_SetText` (`self.TextRender_Children`) (`self.GetChildText`))
  (`/Engine/EditorBlueprintResources/ActorMacros.Switch Has Authority`
    (:`Authority`
      (bind (_asynctaskproxy _payload) (`AbilityAsync_WaitGameplayEvent.WaitGameplayEventToActor` null (`SelectionComponent.SelectionTag` (`self.ValidationComponent`)) false false)
        (:`EventReceived`
          (`self.UpdateTextRenderer` _payload))))))

(event `UpdateTextRenderer`
  (params (Payload :type "GameplayEventData Structure"))
  (bind _childtext (`self.GetSelectablesInfoToText` (`ValidationComponent.GetAllSelectablesInfo` (`self.ValidationComponent`))))
  (if (not (`KismetArrayLibrary.Array_Identical` (`self.ChildTexts`) _childtext))
    (set `self.ChildTexts` _childtext)
    (`TextRenderComponent.K2_SetText` (`self.TextRender_Children`) (`self.GetChildText`))))

(event `self.ReceiveTick`
  (params (DeltaSeconds :type "Float (single-precision)"))
  (bind (_baseduration _remainingduration _rate _evaluationtag _evaluationtimerhandle) (break `SelectionEvaluation` (`ValidationComponent.SelectionEvaluation` (`self.ValidationComponent`))))
  (`parent.ReceiveTick` DeltaSeconds)
  (if (`KismetSystemLibrary.K2_IsTimerActiveHandle` _evaluationtimerhandle)
    (`TextRenderComponent.K2_SetText` (`self.TextRender_Timer`) (`|FormatText` "Handles {tag} in: {time} " (`BlueprintGameplayTagLibrary.GetTagName` _evaluationtag) (`KismetMathLibrary.FCeil` _remainingduration)))
    (if (not (`SceneComponent.bVisible` (`self.TextRender_Timer`)))
      (`SceneComponent.SetVisibility` (`self.TextRender_Timer`) true true))
    (elif (`SceneComponent.bVisible` (`self.TextRender_Timer`))
      (`SceneComponent.SetVisibility` (`self.TextRender_Timer`) false true))))

(fn `GetSelectablesInfoToText`
  (params (SelectableInfos :type "Array of SelectablesInfo Structure"))
  (returns (ChildText :type "Array of String"))
  (locals (Texts :type "Array of String"))
  (for _array_element SelectableInfos
    (`KismetArrayLibrary.Array_Add` (`local.Texts`) (`KismetStringLibrary.Conv_IntToString` (`.TotalSelectors` (break `SelectablesInfo` _array_element)))))
  (return (`local.Texts`)))

(fn `OnRep_ChildTexts`
  (`TextRenderComponent.K2_SetText` (`self.TextRender_Children`) (`self.GetChildText`)))

(fn `UserConstructionScript`)