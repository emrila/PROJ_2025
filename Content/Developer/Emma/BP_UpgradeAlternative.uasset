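; Upgrade option that pops out of its owning chest as a spinning, interactable object and retracts on close.
; On the server, the owner's open and close events trigger randomly staggered multicasts, with closing limited to zero selectors or invalid selection info.
; Timelines move it between chest and original position and fade its light and widget.
; Sphere collision determines interactability and is disabled by the Locked tag or closing.
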(event `self.ReceiveBeginPlay`
  (`parent.ReceiveBeginPlay`)
  (`PrimitiveComponent.SetCollisionEnabled` (`self.SphereComponent`) "NoCollision")
  ;[0.1667 0 1 0.2] On Lock Tag Added (through Gameplay Effect)
  (`AbilityAsync_WaitGameplayTagAdded.WaitGameplayTagAddToActor` null (struct :`TagName` "Selection.State.Locked")
    (:`then`
      (`AbilityAsync_WaitGameplayEvent.WaitGameplayEventToActor` (`self.GetOwner`) (struct :`TagName` "Event.Object.Open")
        (:`then`
          (`AbilityAsync_WaitGameplayEvent.WaitGameplayEventToActor` (`self.GetOwner`) (struct :`TagName` "Event.Object.Close")
            (:`then`
              (set `self.DefaultWorldPosition` (`self.K2_GetActorLocation`))
              (`SceneComponent.SetVisibility` (`self.StaticMeshComponent`) false false)
              (`WidgetComponent.SetTintColorAndOpacity` (`self.WidgetComponent`) (struct :`R` 1.0 :`G` 1.0 :`B` 1.0))
              (set `self.LightIntensity` (`LightComponentBase.Intensity` (`self.PointLight`)))
              (`LightComponent.SetIntensity` (`self.PointLight`) 0.0)
              (`self.Rotate`))
            (:`EventReceived`
              (`/Engine/EditorBlueprintResources/ActorMacros.Switch Has Authority`
                (:`Authority`
                  (bind _returnvalue (`SelectionDisplayInterface.OnGetSelectablesInfo` null))
                  (bind _value (`BlueprintInstancedStructLibrary.GetInstancedStructValue` _returnvalue)
                    (:`Valid`
                      (if (== (`.TotalSelectors` (break `SelectablesInfo` _value)) 0)
                        (`KismetSystemLibrary.K2_SetTimerDelegate` (delegate `CloseEvent`) 2.0 :!label _label)
                        (`self.Multicast_PreCloseChest`)))
                    (:`NotValid`
                      (goto _label))))))))
        (:`EventReceived`
          (`/Engine/EditorBlueprintResources/ActorMacros.Switch Has Authority`
            (:`Authority`
              (`KismetSystemLibrary.K2_SetTimerDelegate` (delegate `OpenEvent`) 2.5)
              (set `self.ParentWorldPosition` (+ (`self.K2_GetActorLocation` (`self.GetOwner`)) (0.0 0.0 80.0)))
              (set `self.DefaultWorldPosition` (`self.K2_GetActorLocation`))
              (`KismetSystemLibrary.Delay` (`KismetMathLibrary.RandomFloatInRange` 1.0 2.25))
              (`self.Multicast_OnChestOpen`))))))
    (:`Added`
      (`PrimitiveComponent.SetCollisionEnabled` (`self.SphereComponent`) "NoCollision"))))

(event `Rotate`
  (bind (_relativerotation_roll _relativerotation_pitch) (`KismetMathLibrary.BreakRotator` (`SceneComponent.RelativeRotation` (`self.StaticMeshComponent`))))
  (bind (_direction _newtrack_0) (`Timeline|Timeline`)
    (:`Update`
      (`SceneComponent.K2_SetRelativeRotation` (`self.StaticMeshComponent`) (`KismetMathLibrary.MakeRotator` _relativerotation_roll _relativerotation_pitch (`KismetMathLibrary.Lerp` 0.0 360.0 _newtrack_0)) false false))))

(event `CloseEvent`
  (`KismetSystemLibrary.Delay` (`KismetMathLibrary.RandomFloatInRange` 0.5 1.5))
  (`self.Multicast_OnChestClosed`))

(event `OpenEvent`
  (`self.Multicast_PostOpenChest`))

(event `Multicast_OnChestOpen`
  (`LightComponent.SetIntensity` (`self.PointLight`) 0.0)
  (`self.K2_SetActorLocation` (`self.ParentWorldPosition`) false true)
  (`SceneComponent.SetVisibility` (`self.StaticMeshComponent`) true true)
  (bind (_direction _force _alpha) (`Timeline|OpenChest_Timeline`)
    (:`Update`
      (`self.LerpLocation` (+ (`self.K2_GetActorLocation`) (`KismetMathLibrary.MakeVector` 0.0 0.0 _force)) (`self.DefaultWorldPosition`) _alpha))))

(event `Multicast_PostOpenChest`
  (`PrimitiveComponent.SetCollisionEnabled` (`self.SphereComponent`) "QueryAndPhysics")
  (bind (_direction _alpha) (`Timeline|PostChestOpen_Timeline`)
    (:`Update`
      (`self.LerpLightIntensity` 0.0 (`self.LightIntensity`) _alpha)
      (`WidgetComponent.SetTintColorAndOpacity` (`self.WidgetComponent`) (make `LinearColor` 1.0 1.0 1.0 _alpha)))))

(event `Multicast_PreCloseChest`
  (`PrimitiveComponent.SetCollisionEnabled` (`self.SphereComponent`) "NoCollision")
  (bind (_direction _alpha) (`Timeline|PreCloseChest_Timeline`)
    (:`Update`
      (`self.LerpLightIntensity` (`self.LightIntensity`) 0.0 _alpha)
      (`WidgetComponent.SetTintColorAndOpacity` (`self.WidgetComponent`) (make `LinearColor` 1.0 1.0 1.0 _alpha)))))

(event `Multicast_OnChestClosed`
  (bind (_direction _alpha) (`Timeline|CloseChest_Timeline`)
    (:`Update`
      (`self.LerpLocation` (`self.K2_GetActorLocation`) (`self.ParentWorldPosition`) _alpha))
    (:`Hide`
      (`SceneComponent.SetVisibility` (`self.StaticMeshComponent`) false false))))

(fn `CanInteract`
  (returns (ReturnValue :type Boolean))
  (return (`PrimitiveComponent.K2_IsCollisionEnabled` (`self.SphereComponent`))))

(fn `LerpLightIntensity`
  (params (A :type "Float (double-precision)") (B :type "Float (double-precision)") (Alpha :type "Float (single-precision)"))
  (`LightComponent.SetIntensity` (`self.PointLight`) (`KismetMathLibrary.Lerp` A B Alpha)))

(fn `LerpLocation`
  (params (A :type "Vector Structure") (B :type "Vector Structure") (Alpha :type "Float (single-precision)"))
  (`self.K2_SetActorLocation` (`KismetMathLibrary.VLerp` A B Alpha) false true))

(fn `UserConstructionScript`)