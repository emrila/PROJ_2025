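; Test selectable, interactable actor that shows a running count of how many times it is selected.
; Select and deselect events go to a server update of CurrentTotal, with an OnRep refreshing both text renderers.
; Proximity gameplay events toggle which of the Enter and Exit texts is visible.
; Adding the Selection.State.Locked tag disables the sphere's collision, which makes CanInteract return false.
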(event `self.ReceiveBeginPlay`
  (`parent.ReceiveBeginPlay`)
  (`AbilityAsync_WaitGameplayTagAdded.WaitGameplayTagAddToActor` null (struct :`TagName` "Selection.State.Locked")
    (:`then`
      (bind (_asynctaskproxy _payload) (`AbilityAsync_WaitGameplayEvent.WaitGameplayEventToActor` null (`InteractableComponent.ProximityTag` (`self.InteractableComponent`)) false false)
        (:`EventReceived`
          (`self.OnChangeTextRenderer` _payload))))
    (:`Added`
      (`PrimitiveComponent.SetCollisionEnabled` (`self.Sphere`) "NoCollision"))))

(event `self.OnSelected`
  (params (Data :type "InstancedStruct Structure"))
  ; ISELECTABLE
  (`parent.OnSelected` Data)
  (bind _value (`BlueprintInstancedStructLibrary.GetInstancedStructValue` Data)
    (:`Valid`
      (`self.Server_UpdateTotal` _value))))

(event `Server_UpdateTotal`
  (params (EventData :type "GameplayEventData Structure"))
  (bind _currenttotal (`self.CurrentTotal`))
  (bind _returnvalue (`KismetTextLibrary.Conv_IntToText` (`self.CurrentTotal`)))
  (`|SwitchGameplayTag` (`.EventTag` (break `GameplayEventData` EventData))
    (:`Selection.Event.Selection.Select`
      (set `self.CurrentTotal` (+ (`self.CurrentTotal`) 1)))
    (:`Selection.Event.Selection.Deselect`
      (set `self.CurrentTotal` (`KismetMathLibrary.Clamp` (- _currenttotal 1) 0 _currenttotal))))
  (`TextRenderComponent.K2_SetText` (`self.TextRender_Exit`) _returnvalue)
  (`TextRenderComponent.K2_SetText` (`self.TextRender_Enter`) _returnvalue))

(event `self.OnDeselected`
  (params (Data :type "InstancedStruct Structure"))
  ; ISELECTABLE
  (`parent.OnDeselected` Data)
  (bind _value (`BlueprintInstancedStructLibrary.GetInstancedStructValue` Data)
    (:`Valid`
      (`self.Server_UpdateTotal` _value))))

(event `OnChangeTextRenderer`
  (params (GameplayEventData :type "GameplayEventData Structure (by ref)"))
  ; IINTERACTABLE
  (`|SwitchGameplayTag` (`.EventTag` (break `GameplayEventData` GameplayEventData))
    (:`Selection.Event.Proximity.Enter`
      (`SceneComponent.SetVisibility` (`self.TextRender_Exit`) false true)
      (`SceneComponent.SetVisibility` (`self.TextRender_Enter`) true true))
    (:`Selection.Event.Proximity.Exit`
      (`SceneComponent.SetVisibility` (`self.TextRender_Exit`) true true)
      (`SceneComponent.SetVisibility` (`self.TextRender_Enter`) false true))))

(fn `CanInteract`
  (returns (ReturnValue :type Boolean))
  (return (`PrimitiveComponent.K2_IsCollisionEnabled` (`self.Sphere`))))

(fn `OnRep_CurrentTotal`
  (bind _returnvalue (`KismetTextLibrary.Conv_IntToText` (`self.CurrentTotal`)))
  (`TextRenderComponent.K2_SetText` (`self.TextRender_Exit`) _returnvalue)
  (`TextRenderComponent.K2_SetText` (`self.TextRender_Enter`) _returnvalue))

(fn `UserConstructionScript`)