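; GA_CloseChest is an event-activated gameplay ability that closes a chest owned by a BP_UpgradeSpawner.
; After a successful commit and a short delay, it multicasts the spawner's animation in reverse and waits for it to complete.
; On completion it applies GE_CloseEffect to the owner and ends, while a failed commit or cast ends the ability immediately.
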(event `self.K2_ActivateAbilityFromEvent`
  (params (EventData :type "GameplayEventData Structure (by ref)"))
  (bind _returnvalue (`self.K2_CommitAbility`))
  (if _returnvalue
    (`KismetSystemLibrary.Delay` 4.0)
    (bind _asbp_upgrade_spawner (cast `/Game/RoomMakerTools/BP_UpgradeSpawner` (`self.GetOwningActorFromActorInfo`))
      (:`then`
        (`/Game/RoomMakerTools/BP_UpgradeSpawner.Multicast_PlayAnimation` _asbp_upgrade_spawner (`self.Animation`) true)
        (`AnimAssetCompleteTask.WaitForAnimationAsset` (`self.Animation`)
          (:`OnComplete`
            (`self.BP_ApplyGameplayEffectToOwner` "/Game/Developer/Emma/Effects/GE_CloseEffect.GE_CloseEffect_C"))))
      (:`CastFailed`
        _)))
  (`self.K2_EndAbility`))