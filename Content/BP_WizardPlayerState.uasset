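; Player state for a wizard game that manages networked voice chat through a VOIPTalker.
; StartVoice tunes mic console settings, applies a voice sound mix and sets the voice mode.
; InitVOIP retries until player state 0 is valid, then registers the talker, choosing attenuation and effects by mode.
; ToggleVoice starts or stops transmission, and CloseVoice mutes, removes remote talkers and clears voice packets.
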(event `StartVoice`
  (bind _returnvalue (`GameplayStatics.GetPlayerController` 0))
  ; Voice
  (`KismetSystemLibrary.ExecuteConsoleCommand` "voice.MicInputGain 3" _returnvalue)
  (`KismetSystemLibrary.ExecuteConsoleCommand` "ToggleSpeaking 0" _returnvalue)
  (`KismetSystemLibrary.ExecuteConsoleCommand` "voice.SilenceDetectionThreshold 0.001" _returnvalue)
  (`KismetSystemLibrary.ExecuteConsoleCommand` "voice.MicNoiseGateThreshold 0.001" _returnvalue)
  (`GameplayStatics.SetBaseSoundMix` "/Game/VoiceChat/SCM_Voice.SCM_Voice")
  (`self.SetVoiceMode` "NewEnumerator1"))

(event `Init VOIP`
  (bind _returnvalue (`GameplayStatics.GetPlayerState` 0))
  ; Voice
  (`/Engine/EditorBlueprintResources/StandardMacros.IsValid` _returnvalue :!label _label
    (:`Is Valid`
      (`VOIPTalker.RegisterWithPlayerState` (`self.VOIPTalker`) _returnvalue)
      (`VOIPStatics.SetMicThreshold` -1.5)
      (set `VOIPTalker.Settings` (select `/Game/VoiceChat/E_Voice` (`self.Voice`) :`NewEnumerator0` (make `VoiceSettings` null) :`NewEnumerator1` (make `VoiceSettings` null "/Game/VoiceChat/SA_Voice.SA_Voice" "/Game/VoiceChat/SEPC_Voice.SEPC_Voice")) (`self.VOIPTalker`))
      (`KismetSystemLibrary.PrintString` "Player Registered"))
    (:`Is Not Valid`
      (`KismetSystemLibrary.RetriggerableDelay` 0.2)
      (goto _label))))

(event `SetVoiceMode`
  (params (Voice :type "/Game/VoiceChat/E_Voice Enum" :default "NewEnumerator0"))
  ; Voice
  (set `self.Voice` Voice))

(event `ToggleVoice`
  (bind _returnvalue (`GameplayStatics.GetPlayerController` 0))
  ; Voice
  (if (`self.bVoiceChatOn`)
    (`self.VOIPTalker`
      (:`then`
        (`AdvancedVoiceLibrary.StopNetworkedVoice` 0)
        (`KismetSystemLibrary.ExecuteConsoleCommand` "ToggleSpeaking 0" _returnvalue)
        (set `self.bVoiceChatOn` false)
        (`KismetSystemLibrary.PrintString` "Ended Voice Chat"))
      (:`else`))
    (else
      (`self.VOIPTalker`
        (:`then`
          (`AdvancedVoiceLibrary.StartNetworkedVoice` 0)
          (`KismetSystemLibrary.ExecuteConsoleCommand` "ToggleSpeaking 1" _returnvalue)
          (set `self.bVoiceChatOn` true)
          (`KismetSystemLibrary.PrintString` "Started Voice Chat"))
        (:`else`)))))

(event `CloseVoice`
  (bind _returnvalue (`GameplayStatics.GetPlayerState` 0))
  ; Voice
  (`self.VOIPTalker`
    (:`then`
      (if (!= (`self.Voice`) 0)
        (`KismetSystemLibrary.ExecuteConsoleCommand` "ToggleSpeaking 0" (`self.GetPlayerController` _returnvalue))
        (`AdvancedVoiceLibrary.MuteRemoteTalker` 0 (`AdvancedSessionsLibrary.GetUniqueNetIDFromPlayerState` _returnvalue) true)
        (`AdvancedVoiceLibrary.RemoveAllRemoteTalkers`)
        (`VoiceLibrary.ClearVoicePackage` self)))
    (:`else`)))

(fn `UserConstructionScript`)