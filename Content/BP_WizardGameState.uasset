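; BP_WizardGameState is the game state for the wizard game, relaying health bar refreshes and votes.
; OnRepHealth calls UpdateHealthbar, which loops over PlayerArray and refreshes each valid Healthbar held by a BP_PlayerControllerBase, stopping if that cast fails.
; Vote passes the candidate to the BP_VotingBooth actor found by class lookup.
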(event `self.OnRep_Health`
  (`self.UpdateHealthbar`))

(event `UpdateHealthbar`
  (for _array_element (`self.PlayerArray`)
    (bind _asbp_player_controller_base (cast `/Game/Developer/Basir/BP_PlayerControllerBase` (`PlayerState.GetPlayerController` _array_element)))
    (bind _healthbar (`/Game/Developer/Basir/BP_PlayerControllerBase.Healthbar` _asbp_player_controller_base))
    (`/Engine/EditorBlueprintResources/StandardMacros.IsValid` _healthbar
      (:`Is Valid`
        (`/Game/UI/Player/WBP_PlayerHealthbar.UpdateHealthbar` _healthbar)))))

(event `Vote`
  (params (Candidate :type "Candidate Structure"))
  (bind _returnvalue (`GameplayStatics.GetActorOfClass` "/Game/Voting/BP_VotingBooth.BP_VotingBooth_C"))
  (`VotingBooth.Vote` _returnvalue Candidate))

(fn `UserConstructionScript`)