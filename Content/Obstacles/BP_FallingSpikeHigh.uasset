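; Falling spike trap obstacle that drops when a player enters its trigger box, then rises back to re-arm.
; The server-side trigger calls Fall, which uses a short delay, a DoOnce gate and two timelines to lower and raise the Cube.
; A second box crushes overlapping players, applying trap damage, squashing their mesh and teleporting them to FlattenLocation.
; A delayed Flatten timeline then animates the squashed mesh's Z scale.
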(event `self.ReceiveBeginPlay`)

(event `self.Box.OnComponentBeginOverlap`
  (params (OverlappedComponent :type "PrimitiveComponent Object Reference") (OtherActor :type "Actor Object Reference") (OtherComp :type "PrimitiveComponent Object Reference") (OtherBodyIndex :type Integer) (bFromSweep :type Boolean) (SweepResult :type "HitResult Structure (by ref)"))
  (if (`self.Active`)
    (cast `/Game/Developer/Basir/BP_PlayerCharacterBase` OtherActor)
    (`/Engine/EditorBlueprintResources/ActorMacros.Switch Has Authority`
      (:`Authority`
        (`self.Fall`)))))

(event `Fall`
  (if (`self.Active`)
    (`KismetSystemLibrary.Delay` 0.5)
    (`/Engine/EditorBlueprintResources/StandardMacros.DoOnce` false :!label _label
      (:`Completed`
        (bind (_direction _newtrack_0) (`Timeline|Timeline` :!via `PlayFromStart`)
          (:`Update`
            (`SceneComponent.K2_SetRelativeLocation` (`self.Cube`) (`KismetMathLibrary.MakeVector` 0.0 0.0 _newtrack_0) false false))
          (:`Finished`
            (`KismetSystemLibrary.Delay` 1.0)
            (bind (_direction_2 _newtrack_0_2) (`Timeline|Timeline_0` :!via `ReverseFromEnd`)
              (:`Update`
                (`SceneComponent.K2_SetRelativeLocation` (`self.Cube`) (`KismetMathLibrary.MakeVector` 0.0 0.0 _newtrack_0_2) false false))
              (:`Finished`
                (goto _label :!via `Reset`)))))))))

(event `self.Box1.OnComponentBeginOverlap`
  (params (OverlappedComponent :type "PrimitiveComponent Object Reference") (OtherActor :type "Actor Object Reference") (OtherComp :type "PrimitiveComponent Object Reference") (OtherBodyIndex :type Integer) (bFromSweep :type Boolean) (SweepResult :type "HitResult Structure (by ref)"))
  (if (`self.Active`)
    (bind _asplayer_character_base (cast `PlayerCharacterBase` OtherActor))
    (`self.Crush` _asplayer_character_base)))

(event `Reset`
  (params (Mesh :type "SceneComponent Object Reference"))
  (`KismetSystemLibrary.Delay` 1.0)
  (bind (_direction _newtrack_0) (`Timeline|Flatten` :!via `PlayFromStart`)
    (:`Update`
      (`SceneComponent.SetWorldScale3D` Mesh (`KismetMathLibrary.MakeVector` 1.0 1.0 _newtrack_0)))))

(event `Crush`
  (params (Player :type "PlayerCharacterBase Object Reference"))
  (bind _mesh (`Character.Mesh` Player))
  (`GameplayStatics.ApplyDamage` Player (`self.Damage`) null null "/Script/PROJ_2025.TrapDamageType")
  (`SceneComponent.SetWorldScale3D` _mesh (1.0 1.0 0.1))
  (`self.K2_SetActorLocation` Player (`SceneComponent.K2_GetComponentLocation` (`self.FlattenLocation`)) false true)
  (`self.Reset` _mesh))

(fn `UserConstructionScript`)