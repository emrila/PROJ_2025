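; Interactable lever obstacle that disables its linked traps when the player uses it.
; A sphere trigger shows or hides a button-prompt widget for the player, and a looping timer keeps that widget facing the camera.
; On interaction it reports finished to the interactor, then, one time only, destroys the prompt and plays a timeline rotating the lever.
; When the timeline finishes, it calls DisableTrap on every entry in Traps.
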(event `self.ReceiveBeginPlay`
  (`KismetSystemLibrary.K2_SetTimer` null "AdjustWidget" 0.01 true true))

(event `AdjustWidget`
  (bind _widget (`self.Widget`))
  (`/Engine/EditorBlueprintResources/StandardMacros.IsValid` _widget
    (:`Is Valid`
      (`SceneComponent.K2_SetWorldRotation` _widget (`KismetMathLibrary.FindLookAtRotation` (`SceneComponent.K2_GetComponentLocation` _widget) (`SceneComponent.K2_GetComponentLocation` (`PlayerCameraManager.TransformComponent` (`GameplayStatics.GetPlayerCameraManager` 0)))) false false))))

(event `self.OnInteract`
  (params (Interactor :type "Object Object Reference"))
  (message `Interactor.OnFinishedInteraction` Interactor self)
  (`self.DisableTrap`))

(event `DisableTrap`
  (`/Engine/EditorBlueprintResources/StandardMacros.DoOnce` false
    (:`Completed`
      (`ActorComponent.K2_DestroyComponent` (`self.Widget`))
      (bind (_direction _rotation) (`Timeline|Timeline` :!via `PlayFromStart`)
        (:`Update`
          (`SceneComponent.K2_SetRelativeRotation` (`self.Lever`) (`KismetMathLibrary.MakeRotator` _rotation) false false))
        (:`Finished`
          (for _array_element (`self.Traps`)
            (`TrapBase.DisableTrap` _array_element)))))))

(event `self.Sphere.OnComponentBeginOverlap`
  (params (OverlappedComponent :type "PrimitiveComponent Object Reference") (OtherActor :type "Actor Object Reference") (OtherComp :type "PrimitiveComponent Object Reference") (OtherBodyIndex :type Integer) (bFromSweep :type Boolean) (SweepResult :type "HitResult Structure (by ref)"))
  (if (== OtherActor (`GameplayStatics.GetPlayerCharacter` 0))
    (`/Engine/EditorBlueprintResources/StandardMacros.IsValid` (`self.Widget`)
      (:`Is Valid`
        (`self.ShowButtonPrompt`)))))

(event `ShowButtonPrompt`
  (`SceneComponent.SetVisibility` (`self.Widget`) true false))

(event `HideButtonPrompt`
  (`SceneComponent.SetVisibility` (`self.Widget`) false false))

(event `self.Sphere.OnComponentEndOverlap`
  (params (OverlappedComponent :type "PrimitiveComponent Object Reference") (OtherActor :type "Actor Object Reference") (OtherComp :type "PrimitiveComponent Object Reference") (OtherBodyIndex :type Integer))
  (if (== OtherActor (`GameplayStatics.GetPlayerCharacter` 0))
    (`/Engine/EditorBlueprintResources/StandardMacros.IsValid` (`self.Widget`)
      (:`Is Valid`
        (`self.HideButtonPrompt`)))))

(fn `CanInteract`
  (returns (ReturnValue :type Boolean))
  (return true))

(fn `UserConstructionScript`)