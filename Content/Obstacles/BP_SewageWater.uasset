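; BP_SewageWater is a sewage water hazard that slows and damages those who wade into it.
; A looping two-second timer applies trap-type damage to every player character overlapping its Piss component.
; Overlap begin and end events on that component lower and restore the actor's CustomTimeDilation, slowing its whole tick rather than just movement.
; The slowdown has no class filter, so it affects any overlapping actor.
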(event `self.ReceiveBeginPlay`
  (`KismetSystemLibrary.K2_SetTimer` null "DealDamage" 2.0 true))

(event `DealDamage`
  (for _array_element (`PrimitiveComponent.GetOverlappingActors` (`self.Piss`) "/Script/PROJ_2025.PlayerCharacterBase")
    (`GameplayStatics.ApplyDamage` _array_element (`self.Damage`) null null "/Script/PROJ_2025.TrapDamageType")))

(event `self.Piss.OnComponentBeginOverlap`
  (params (OverlappedComponent :type "PrimitiveComponent Object Reference") (OtherActor :type "Actor Object Reference") (OtherComp :type "PrimitiveComponent Object Reference") (OtherBodyIndex :type Integer) (bFromSweep :type Boolean) (SweepResult :type "HitResult Structure (by ref)"))
  (set `Actor.CustomTimeDilation` 0.85 OtherActor))

(event `self.Piss.OnComponentEndOverlap`
  (params (OverlappedComponent :type "PrimitiveComponent Object Reference") (OtherActor :type "Actor Object Reference") (OtherComp :type "PrimitiveComponent Object Reference") (OtherBodyIndex :type Integer))
  (set `Actor.CustomTimeDilation` 1.0 OtherActor))

(fn `UserConstructionScript`)