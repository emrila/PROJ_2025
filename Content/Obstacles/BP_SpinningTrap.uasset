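; Spinning trap obstacle that damages actors touching it and knocks player characters away.
; Tick rolls Cylinder1 by RotationSpeed every frame without delta-time scaling, with FlipRotation reversing the direction.
; Two capsule overlap events call Damage, which applies fixed damage, then launches any PlayerCharacterBase upward and along the trap's negative right vector, regardless of contact side.
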(event `self.ReceiveTick`
  (params (DeltaSeconds :type "Float (single-precision)"))
  (bind _rotationspeed (`self.RotationSpeed`))
  (bind _cylinder1 (`self.Cylinder1`))
  (if (not (`self.FlipRotation`))
    (`SceneComponent.K2_AddLocalRotation` _cylinder1 (`KismetMathLibrary.MakeRotator` _rotationspeed) false false)
    (else
      (`SceneComponent.K2_AddLocalRotation` _cylinder1 (`KismetMathLibrary.MakeRotator` (* _rotationspeed -1.0)) false false))))

(event `self.Capsule.OnComponentBeginOverlap`
  (params (OverlappedComponent :type "PrimitiveComponent Object Reference") (OtherActor :type "Actor Object Reference") (OtherComp :type "PrimitiveComponent Object Reference") (OtherBodyIndex :type Integer) (bFromSweep :type Boolean) (SweepResult :type "HitResult Structure (by ref)"))
  (`self.Damage` OtherActor))

(event `self.Capsule1.OnComponentBeginOverlap`
  (params (OverlappedComponent :type "PrimitiveComponent Object Reference") (OtherActor :type "Actor Object Reference") (OtherComp :type "PrimitiveComponent Object Reference") (OtherBodyIndex :type Integer) (bFromSweep :type Boolean) (SweepResult :type "HitResult Structure (by ref)"))
  (`self.Damage` OtherActor))

(fn `Damage`
  (params (DamagedActor :type "Actor Object Reference"))
  (bind (_returnvalue_x _returnvalue_y) (`KismetMathLibrary.BreakVector` (* (`self.GetActorRightVector`) -500.0)))
  (`GameplayStatics.ApplyDamage` DamagedActor 10.0)
  (bind _asplayer_character_base (cast `PlayerCharacterBase` DamagedActor))
  (`Character.LaunchCharacter` _asplayer_character_base (`KismetMathLibrary.MakeVector` _returnvalue_x _returnvalue_y 200.0) false false))

(fn `UserConstructionScript`)