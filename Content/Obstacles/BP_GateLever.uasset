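; Interactable lever actor that opens a referenced gate when a player or other interactor uses it.
; Interaction immediately reports completion to the interactor, then triggers the opening only on the authority.
; A DoOnce limits it to a single pull: a timeline rotates the lever's roll, then calls OpenGate on the gate when finished.
; CanInteract always returns true, even after the lever is used.
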(event `self.OnInteract`
  (params (Interactor :type "Object Object Reference"))
  (message `Interactor.OnFinishedInteraction` Interactor self)
  (`/Engine/EditorBlueprintResources/ActorMacros.Switch Has Authority`
    (:`Authority`
      (`self.OpenGate`))))

(event `OpenGate`
  (`/Engine/EditorBlueprintResources/StandardMacros.DoOnce` false
    (:`Completed`
      (bind (_direction _rotation) (`Timeline|Timeline` :!via `PlayFromStart`)
        (:`Update`
          (`SceneComponent.K2_SetRelativeRotation` (`self.Lever`) (`KismetMathLibrary.MakeRotator` _rotation) false false))
        (:`Finished`
          (`/Game/Obstacles/BP_Gate.OpenGate` (`self.Gate`)))))))

(fn `CanInteract`
  (returns (ReturnValue :type Boolean))
  (return true))

(fn `UserConstructionScript`)