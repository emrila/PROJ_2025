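; BP_Beam is a beam trap obstacle that damages whatever blocks its line of fire.
; A looping timer, limited to once per frame, line traces forward up to Range while Active and applies trap-type damage to the hit actor.
; A collision-free cylinder serves as the beam, stretched to the hit distance or full range and shrunk to near zero when inactive.
; A SetMaterial event swaps the cylinder's material.
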(event `self.ReceiveBeginPlay`
  (`KismetSystemLibrary.K2_SetTimerDelegate` (delegate `DealDamage`) 0.01 true true)
  (`PrimitiveComponent.SetCollisionEnabled` (`self.Cylinder`) "NoCollision"))

(event `DealDamage`
  (bind _cylinder (`self.Cylinder`))
  (if (`self.Active`)
    (bind _outhit (`KismetSystemLibrary.LineTraceSingle` (`self.K2_GetActorLocation`) (+ (`self.K2_GetActorLocation`) (* (`self.GetActorForwardVector`) (`self.Range`))) "TraceTypeQuery1"))
    (bind (_bblockinghit _binitialoverlap _time _distance _location _impactpoint _normal _impactnormal _physmat _hitactor _hitcomponent _hitbonename _bonename _hititem _elementindex _faceindex _tracestart) (`GameplayStatics.BreakHitResult` _outhit))
    (if _bblockinghit
      (`SceneComponent.SetRelativeScale3D` _cylinder (`KismetMathLibrary.MakeVector` 0.1 0.1 (/ (`KismetMathLibrary.VSize` (- _location _tracestart)) 100.0)))
      (`GameplayStatics.ApplyDamage` _hitactor (`self.Damage`) null null "/Script/PROJ_2025.TrapDamageType")
      (else
        (`SceneComponent.SetRelativeScale3D` _cylinder (`KismetMathLibrary.MakeVector` 0.1 0.1 (/ (`self.Range`) 100.0)))))
    (else
      (`SceneComponent.SetRelativeScale3D` (`self.Cylinder`) (0.001 0.001 0.001)))))

(event `SetMaterial`
  (params (NewMaterial :type "Material Object Reference"))
  (`PrimitiveComponent.SetMaterial` (`self.Cylinder`) 0 NewMaterial))

(fn `UserConstructionScript`)