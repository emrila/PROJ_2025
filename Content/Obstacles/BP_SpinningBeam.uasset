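; BP_SpinningBeam is a trap obstacle that spins a cylinder, with four BP_Beam child actors that receive its Damage value at construction.
; A server-only looping timer rotates the cylinder on yaw, or on negated roll when FlipRotation is set.
; When inactive, it calls Stop to clear the child actor classes.
; DealDamage applies trap damage and launches player characters sideways, but is not called within this Blueprint.
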(event `self.ReceiveBeginPlay`
  (`/Engine/EditorBlueprintResources/ActorMacros.Switch Has Authority`
    (:`Authority`
      (`KismetSystemLibrary.K2_SetTimer` null "Spin" 0.01 true true))))

(event `Spin`
  (bind _rotationspeed (`self.RotationSpeed`))
  (bind _cylinder (`self.Cylinder`))
  (if (`self.Active`)
    (if (not (`self.FlipRotation`))
      (`SceneComponent.K2_AddLocalRotation` _cylinder (`KismetMathLibrary.MakeRotator` 0.0 0.0 _rotationspeed) false false)
      (else
        (`SceneComponent.K2_AddLocalRotation` _cylinder (`KismetMathLibrary.MakeRotator` (* _rotationspeed -1.0)) false false)))
    (else
      (`self.Stop`))))

(event `Stop`
  (`ChildActorComponent.SetChildActorClass` (`self.ChildActor1`) null)
  (`ChildActorComponent.SetChildActorClass` (`self.ChildActor2`) null)
  (`ChildActorComponent.SetChildActorClass` (`self.ChildActor3`) null)
  (`ChildActorComponent.SetChildActorClass` (`self.ChildActor`) null))

(fn `DealDamage`
  (params (DamagedActor :type "Actor Object Reference"))
  (bind (_returnvalue_x _returnvalue_y) (`KismetMathLibrary.BreakVector` (* (`self.GetActorRightVector`) -500.0)))
  (`GameplayStatics.ApplyDamage` DamagedActor (`self.Damage`) null null "/Script/PROJ_2025.TrapDamageType")
  (bind _asplayer_character_base (cast `PlayerCharacterBase` DamagedActor))
  (`Character.LaunchCharacter` _asplayer_character_base (`KismetMathLibrary.MakeVector` _returnvalue_x _returnvalue_y) false false))

(fn `UserConstructionScript`
  (bind _asbp_beam (cast `/Game/Obstacles/BP_Beam` (`ChildActorComponent.ChildActor` (`self.ChildActor1`))))
  (set `/Game/Obstacles/BP_Beam.Damage` (`self.Damage`) _asbp_beam)
  (bind _asbp_beam_2 (cast `/Game/Obstacles/BP_Beam` (`ChildActorComponent.ChildActor` (`self.ChildActor2`))))
  (set `/Game/Obstacles/BP_Beam.Damage` (`self.Damage`) _asbp_beam_2)
  (bind _asbp_beam_3 (cast `/Game/Obstacles/BP_Beam` (`ChildActorComponent.ChildActor` (`self.ChildActor3`))))
  (set `/Game/Obstacles/BP_Beam.Damage` (`self.Damage`) _asbp_beam_3)
  (bind _asbp_beam_4 (cast `/Game/Obstacles/BP_Beam` (`ChildActorComponent.ChildActor` (`self.ChildActor`))))
  (set `/Game/Obstacles/BP_Beam.Damage` (`self.Damage`) _asbp_beam_4))