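; Swinging axe obstacle that oscillates like a pendulum, damaging and knocking back what it hits.
; Each Tick it speeds up or slows down based on the Anchor's pitch against DeaccelerationAngle and swing direction, then rotates the Anchor.
; Reaching MaxAngle on either side flips direction and zeroes speed.
; Box overlap applies damage and launches BP_PlayerCharacterBase actors along the axe's negative right vector, regardless of swing direction.
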(event `self.ReceiveTick`
  (params (DeltaSeconds :type "Float (single-precision)"))
  (bind _returnvalue (`self.ShouldAccelerate?`))
  (if _returnvalue
    (`self.Accelerate` DeltaSeconds)
    (else
      (`self.Deaccelerate` DeltaSeconds)))
  (`self.Rotate` DeltaSeconds))

(event `self.Box.OnComponentBeginOverlap`
  (params (OverlappedComponent :type "PrimitiveComponent Object Reference") (OtherActor :type "Actor Object Reference") (OtherComp :type "PrimitiveComponent Object Reference") (OtherBodyIndex :type Integer) (bFromSweep :type Boolean) (SweepResult :type "HitResult Structure (by ref)"))
  (bind (_returnvalue_x _returnvalue_y) (`KismetMathLibrary.BreakVector` (* (`self.GetActorRightVector`) -500.0)))
  (`GameplayStatics.ApplyDamage` OtherActor (`self.Damage`))
  (bind _asbp_player_character_base (cast `/Game/Developer/Basir/BP_PlayerCharacterBase` OtherActor))
  (`Character.LaunchCharacter` _asbp_player_character_base (`KismetMathLibrary.MakeVector` _returnvalue_x _returnvalue_y 0.0) false false))

(fn `Accelerate`
  (params (DeltaTime :type "Float (double-precision)"))
  (if (< (`self.CurrentRotationSpeed`) (`self.MaxRotationSpeed`))
    (set `self.CurrentRotationSpeed` (+ (`self.CurrentRotationSpeed`) (* (`self.RotationAcceleration`) DeltaTime)))
    (else
      (set `self.CurrentRotationSpeed` (`self.MaxRotationSpeed`)))))

(fn `Deaccelerate`
  (params (DeltaTime :type "Float (double-precision)"))
  (if (> (`self.CurrentRotationSpeed`) 30.0)
    (set `self.CurrentRotationSpeed` (- (`self.CurrentRotationSpeed`) (* (`self.RotationDeacceleration`) DeltaTime)))
    (else
      (set `self.CurrentRotationSpeed` (`self.MinimumRotationSpeed`)))))

(fn `Rotate`
  (params (DeltaTime :type "Float (double-precision)"))
  (bind _anchor (`self.Anchor`))
  (bind (_returnvalue_roll _returnvalue_pitch) (`KismetMathLibrary.BreakRotator` (`SceneComponent.K2_GetComponentRotation` (`self.Anchor`))))
  (bind (_returnvalue_roll_2 _returnvalue_pitch_2) (`KismetMathLibrary.BreakRotator` (`SceneComponent.K2_GetComponentRotation` (`self.Anchor`))))
  (if (`self.MoveForward?`)
    (`SceneComponent.K2_AddLocalRotation` _anchor (`KismetMathLibrary.MakeRotator` 0.0 (* DeltaTime (`self.CurrentRotationSpeed`))) false false)
    (if (>= _returnvalue_pitch_2 (`self.MaxAngle`))
      (set `self.MoveForward?` false)
      (set `self.CurrentRotationSpeed` 0.0 :!label _label))
    (else
      (`SceneComponent.K2_AddLocalRotation` _anchor (`KismetMathLibrary.MakeRotator` 0.0 (* (* (`self.CurrentRotationSpeed`) -1.0) DeltaTime)) false false)
      (if (<= _returnvalue_pitch (* (`self.MaxAngle`) -1.0))
        (set `self.MoveForward?` true)
        (goto _label)))))

(fn `ShouldAccelerate?`
  (returns (ReturnValue :type Boolean))
  (bind (_returnvalue_roll _returnvalue_pitch) (`KismetMathLibrary.BreakRotator` (`SceneComponent.K2_GetComponentRotation` (`self.Anchor`))))
  (bind (_returnvalue_roll_2 _returnvalue_pitch_2) (`KismetMathLibrary.BreakRotator` (`SceneComponent.K2_GetComponentRotation` (`self.Anchor`))))
  (return (or (and (>= _returnvalue_pitch (`self.DeaccelerationAngle`)) (not (`self.MoveForward?`))) (and (<= _returnvalue_pitch_2 (* (`self.DeaccelerationAngle`) -1.0)) (`self.MoveForward?`)))))

(fn `UserConstructionScript`)