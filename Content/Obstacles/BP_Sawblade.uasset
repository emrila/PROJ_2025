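; Sawblade obstacle that spins and shuttles back and forth along a trail, damaging any Character overlapping the blade.
; The construction script sizes the trail from Length by placing both end pieces, stretching and tiling a spline mesh, and positioning the blade at Progress.
; A fast looping timer, rather than Tick, drives Move, which applies Damage on every step and ping-pongs Progress by Speed to lerp the blade between the ends.
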(event `self.ReceiveBeginPlay`
  (`KismetSystemLibrary.K2_SetTimer` null "Move" 0.01 true))

(event `Move`
  (for _array_element (`PrimitiveComponent.GetOverlappingActors` (`self.SM_SawBlade`) "/Script/Engine.Character")
    (`GameplayStatics.ApplyDamage` _array_element (`self.Damage`)))
  (`SceneComponent.K2_AddLocalRotation` (`self.SM_SawBlade`) (struct :`Pitch` 5.0) false false)
  (if (`self.GoForward`)
    (set `self.Progress` (`KismetMathLibrary.FClamp` (+ (* (`self.Speed`) 0.01) (`self.Progress`))))
    (`SceneComponent.K2_SetRelativeLocation` (`self.SM_SawBlade`) (`KismetMathLibrary.VLerp` (+ (`SceneComponent.RelativeLocation` (`self.SM_SawBlade_Trail_Right_3x3m`)) (200.0 -150.0 0.0)) (+ (`SceneComponent.RelativeLocation` (`self.SM_SawBlade_Trail_Left_3x3m`)) (100.0 -150.0 0.0)) (`self.Progress`)) false false)
    (if (== (`self.Progress`) 1.0)
      (set `self.GoForward` false))
    (else
      (set `self.Progress` (`KismetMathLibrary.FClamp` (- (`self.Progress`) (* (`self.Speed`) 0.01))))
      (`SceneComponent.K2_SetRelativeLocation` (`self.SM_SawBlade`) (`KismetMathLibrary.VLerp` (+ (`SceneComponent.RelativeLocation` (`self.SM_SawBlade_Trail_Right_3x3m`)) (200.0 -150.0 0.0)) (+ (`SceneComponent.RelativeLocation` (`self.SM_SawBlade_Trail_Left_3x3m`)) (100.0 -150.0 0.0)) (`self.Progress`)) false false)
      (if (== (`self.Progress`) 0.0)
        (set `self.GoForward` true)))))

(fn `UserConstructionScript`
  (locals (NewLocalVar :type "Vector Structure" :default (0.0 1.0 0.01)))
  (bind _splinemesh (`self.SplineMesh`))
  (`MeshComponent.SetScalarParameterValueOnMaterials` (`self.SplineMesh`) "TileAmount" (`KismetMathLibrary.Conv_IntToDouble` (`self.Length`)))
  (`SceneComponent.K2_SetRelativeLocation` (`self.SM_SawBlade_Trail_Right_3x3m`) (`KismetMathLibrary.MakeVector` (* 150.0 (`self.Length`)) 150.0) false false)
  (`SceneComponent.K2_SetRelativeLocation` (`self.SM_SawBlade_Trail_Left_3x3m`) (`KismetMathLibrary.MakeVector` (* -150.0 (`self.Length`)) 150.0) false false)
  (`SplineMeshComponent.SetStartPosition` _splinemesh (- (`SceneComponent.RelativeLocation` (`self.SM_SawBlade_Trail_Left_3x3m`)) (-300.0 150.0 0.0)) true)
  (`SplineMeshComponent.SetEndPosition` _splinemesh (- (`SceneComponent.RelativeLocation` (`self.SM_SawBlade_Trail_Right_3x3m`)) (0.0 150.0 0.0)) true)
  (`SceneComponent.K2_SetRelativeLocation` (`self.SM_SawBlade`) (`KismetMathLibrary.VLerp` (+ (`SceneComponent.RelativeLocation` (`self.SM_SawBlade_Trail_Right_3x3m`)) (0.0 -150.0 0.0)) (+ (`SceneComponent.RelativeLocation` (`self.SM_SawBlade_Trail_Left_3x3m`)) (0.0 -150.0 0.0)) (`self.Progress`)) false false))