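; BP_FallingSpike is an obstacle that drops when a player enters its trigger box, then retracts.
; A DoOnce gates two timelines that move the cube along Z from its start location, with delays before falling and retracting.
; A second box applies environmental damage, squashes the player's mesh and teleports the player to FlattenLocation.
; After a delay, the Flatten timeline animates the mesh's Z scale.
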(event `self.ReceiveBeginPlay`
  (set `self.StartLocation` (`SceneComponent.K2_GetComponentLocation` (`self.Cube`))))

(event `self.Box.OnComponentBeginOverlap`
  (params (OverlappedComponent :type "PrimitiveComponent Object Reference") (OtherActor :type "Actor Object Reference") (OtherComp :type "PrimitiveComponent Object Reference") (OtherBodyIndex :type Integer) (bFromSweep :type Boolean) (SweepResult :type "HitResult Structure (by ref)"))
  (cast `/Game/Developer/Basir/BP_PlayerCharacterBase` OtherActor)
  (`self.Fall`))

(event `Fall`
  (`KismetSystemLibrary.Delay` 0.5)
  (`/Engine/EditorBlueprintResources/StandardMacros.DoOnce` false :!label _label
    (:`Completed`
      (bind (_direction _newtrack_0) (`Timeline|Timeline` :!via `PlayFromStart`)
        (:`Update`
          (`SceneComponent.K2_SetWorldLocation` (`self.Cube`) (+ (`self.StartLocation`) (`KismetMathLibrary.MakeVector` 0.0 0.0 _newtrack_0)) false false))
        (:`Finished`
          (`KismetSystemLibrary.Delay` 1.0)
          (bind (_direction_2 _newtrack_0_2) (`Timeline|Timeline_1` :!via `ReverseFromEnd`)
            (:`Update`
              (`SceneComponent.K2_SetWorldLocation` (`self.Cube`) (+ (`self.StartLocation`) (`KismetMathLibrary.MakeVector` 0.0 0.0 _newtrack_0_2)) false false))
            (:`Finished`
              (goto _label :!via `Reset`))))))))

(event `self.Box1.OnComponentBeginOverlap`
  (params (OverlappedComponent :type "PrimitiveComponent Object Reference") (OtherActor :type "Actor Object Reference") (OtherComp :type "PrimitiveComponent Object Reference") (OtherBodyIndex :type Integer) (bFromSweep :type Boolean) (SweepResult :type "HitResult Structure (by ref)"))
  (bind _asplayer_character_base (cast `PlayerCharacterBase` OtherActor))
  (`GameplayStatics.ApplyDamage` _asplayer_character_base 1.0 null null "/Engine/EngineDamageTypes/DmgTypeBP_Environmental.DmgTypeBP_Environmental_C")
  (bind _mesh (`Character.Mesh` _asplayer_character_base))
  (`SceneComponent.SetWorldScale3D` _mesh (1.0 1.0 0.1))
  (`self.K2_SetActorLocation` OtherActor (`SceneComponent.K2_GetComponentLocation` (`self.FlattenLocation`)) false true)
  (`self.Reset` _mesh)
  (bind (_direction _newtrack_0) (`Timeline|Flatten` :!via `Stop` :!label _label_2)
    (:`Update`
      (`SceneComponent.SetWorldScale3D` (stale `Reset` Mesh) (`KismetMathLibrary.MakeVector` 1.0 1.0 _newtrack_0)))))

(event `Reset`
  (params (Mesh :type "SceneComponent Object Reference"))
  (`KismetSystemLibrary.Delay` 4.0)
  (goto _label_2 :!via `PlayFromStart`))

(fn `UserConstructionScript`)