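; Lobby game mode that sets up voice chat as players join.
; PostLogin and HandleStartingNewPlayer run the same logic: cast the new player to BP_PlayerControllerBase and call StartVoice on it.
; Each then loops over the GameState PlayerArray and calls InitVOIP on every player's controller, so existing players are re-initialised on each arrival.
; HandleStartingNewPlayer calls its parent implementation first.
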(event `self.K2_PostLogin`
  (params (NewPlayer :type "PlayerController Object Reference"))
  (bind _asbp_player_controller_base (cast `/Game/Developer/Basir/BP_PlayerControllerBase` NewPlayer))
  (`/Game/Developer/Basir/BP_PlayerControllerBase.StartVoice` _asbp_player_controller_base)
  (for _array_element (`GameStateBase.PlayerArray` (`GameplayStatics.GetGameState`))
    (bind _asbp_player_controller_base_2 (cast `/Game/Developer/Basir/BP_PlayerControllerBase` (`PlayerState.GetPlayerController` _array_element)))
    (`/Game/Developer/Basir/BP_PlayerControllerBase.Init VOIP` _asbp_player_controller_base_2)))

(event `self.HandleStartingNewPlayer`
  (params (NewPlayer :type "PlayerController Object Reference"))
  (`parent.HandleStartingNewPlayer` NewPlayer)
  (bind _asbp_player_controller_base (cast `/Game/Developer/Basir/BP_PlayerControllerBase` NewPlayer))
  (`/Game/Developer/Basir/BP_PlayerControllerBase.StartVoice` _asbp_player_controller_base)
  (for _array_element (`GameStateBase.PlayerArray` (`GameplayStatics.GetGameState`))
    (bind _asbp_player_controller_base_2 (cast `/Game/Developer/Basir/BP_PlayerControllerBase` (`PlayerState.GetPlayerController` _array_element)))
    (`/Game/Developer/Basir/BP_PlayerControllerBase.Init VOIP` _asbp_player_controller_base_2)))

(fn `UserConstructionScript`)